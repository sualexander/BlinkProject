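; BP_DestructableTest is a test prop that breaks when hit hard enough.
; On a StaticMesh hit, it compares the normal impulse magnitude to DamageThreshold and prints the value when exceeded.
; The first such hit, gated by DoOnce, destroys the mesh component and spawns a BP_FlowerPot at the mesh's location and rotation.
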(event `self.StaticMesh.OnComponentHit`
  (params (HitComponent :type "PrimitiveComponent Object Reference") (OtherActor :type "Actor Object Reference") (OtherComp :type "PrimitiveComponent Object Reference") (NormalImpulse :type "Vector Structure") (Hit :type "HitResult Structure (by ref)"))
  (bind _returnvalue (`KismetMathLibrary.VSize` NormalImpulse))
  (bind _staticmesh (`self.StaticMesh`))
  (if (> _returnvalue (`self.DamageThreshold`))
    (`KismetSystemLibrary.PrintString` (`KismetStringLibrary.Conv_DoubleToString` _returnvalue))
    (`/Engine/EditorBlueprintResources/StandardMacros.DoOnce` false
      (:`Completed`
        (bind _output_get (set `self.TempTransform` (`SceneComponent.K2_GetComponentToWorld` _staticmesh)))
        (`ActorComponent.K2_DestroyComponent` _staticmesh)
        (`|SpawnActorFromClass` "/Game/Blueprints/Props/BP_FlowerPot.BP_FlowerPot_C" (`KismetMathLibrary.MakeTransform` (.location _output_get) (.rotation _output_get)) "Undefined" "OverrideRootScale" null null)))))

(fn `UserConstructionScript`)