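; Moving light prop that slides a rect light repeatedly along a path and drives two rising pedestals with spotlights.
; BeginPlay hides the lights and starts a timeline that raises both pedestal meshes, then reveals the spotlights when finished.
; A Turn "On" signal shows the rect light and enables Tick, which lerps it between two locations, snapping back to loop.
; The first Box overlap hides it, stops Tick and replays the timeline after a short delay.
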(event `self.ReceiveBeginPlay`
  (bind _pedestal1 (`self.Pedestal1`))
  (bind _pedestal2 (`self.Pedestal2`))
  (set `self.Location1` (`SceneComponent.K2_GetComponentLocation` (`self.RectLight`)))
  (`SceneComponent.SetHiddenInGame` (`self.RectLight`) true false)
  (set `self.Pedestal1` (`SceneComponent.K2_GetComponentLocation` (`self.StaticMesh1`)))
  (set `self.Pedestal2` (`SceneComponent.K2_GetComponentLocation` (`self.StaticMesh2`)))
  (for _array_element (`self.Lights`)
    (`SceneComponent.SetVisibility` (`SpotLight.SpotLightComponent` _array_element) false false)
    (bind (_direction _height) (`Timeline|Timeline` :!label _label)
      (:`Update`
        (`SceneComponent.K2_SetWorldLocation` (`self.StaticMesh1`) (`KismetMathLibrary.VLerp` _pedestal1 (+ _pedestal1 (0.0 0.0 150.0)) _height) false true)
        (`SceneComponent.K2_SetWorldLocation` (`self.StaticMesh2`) (`KismetMathLibrary.VLerp` _pedestal2 (+ _pedestal2 (0.0 0.0 150.0)) _height) false true))
      (:`Finished`
        (for _array_element_2 (`self.Lights`)
          (`SceneComponent.SetVisibility` (`SpotLight.SpotLightComponent` _array_element_2) true false))))))

(event `/Game/Blueprints/BI_Signal.Turn`
  (params (Signal :type "/Game/FPSPuzzleSP/Blueprints/Components/Enum_Signal Enum" :default "NewEnumerator0"))
  (switch `/Game/FPSPuzzleSP/Blueprints/Components/Enum_Signal` Signal
    (:`NewEnumerator0`
      (`SceneComponent.SetHiddenInGame` (`self.RectLight`) false false)
      (`self.SetActorTickEnabled` true))))

(event `self.ReceiveTick`
  (params (DeltaSeconds :type "Float (single-precision)"))
  (bind _location2 (`self.Location2`))
  (bind _rectlight (`self.RectLight`))
  (bind _returnvalue (`KismetMathLibrary.VLerp` (`self.Location1`) _location2 (`self.Alpha`)))
  (if (== _returnvalue _location2 :`ErrorTolerance` 1.0)
    (`SceneComponent.K2_SetWorldLocation` _rectlight (`self.Location1`) false true)
    (set `self.Alpha` 0.0)
    (else
      (`SceneComponent.K2_SetWorldLocation` _rectlight _returnvalue false true)
      (set `self.Alpha` (+ (`self.Alpha`) (`self.Speed`))))))

(event `self.Box.OnComponentBeginOverlap`
  (params (OverlappedComponent :type "PrimitiveComponent Object Reference") (OtherActor :type "Actor Object Reference") (OtherComp :type "PrimitiveComponent Object Reference") (OtherBodyIndex :type Integer) (bFromSweep :type Boolean) (SweepResult :type "HitResult Structure (by ref)"))
  (`/Engine/EditorBlueprintResources/StandardMacros.DoOnce` false
    (:`Completed`
      (`SceneComponent.SetHiddenInGame` (`self.RectLight`) true false)
      (`self.SetActorTickEnabled` false)
      (`KismetSystemLibrary.Delay` 0.5)
      (goto _label))))

(fn `UserConstructionScript`)