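; Prop spawner that drops random falling objects, apparently to demo emancipation.
; While IsOn, Drop spawns a BP_FallingObject at the actor's location with random rotation and reduced scale, a random mesh from Types and physics enabled.
; Each drop sets a randomly delayed one-shot timer, presumably to repeat itself.
; Drop runs on BeginPlay and from Enable/Disable, which sets IsOn without clearing pending timers.
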(event `self.ReceiveBeginPlay`
  (`self.Drop`))

(event `Drop`
  (if (`self.IsOn`)
    (bind _returnvalue (`|SpawnActorFromClass` "/Game/Blueprints/Props/BP_FallingObject.BP_FallingObject_C" (`KismetMathLibrary.MakeTransform` (`self.K2_GetActorLocation`) (`KismetMathLibrary.RandomRotator` true) (0.75 0.75 0.75)) "Undefined" "OverrideRootScale" null null))
    (bind _staticmesh (`/Game/Blueprints/Props/BP_FallingObject.StaticMesh` _returnvalue))
    (`StaticMeshComponent.SetStaticMesh` _staticmesh (`KismetArrayLibrary.Array_Random` (`self.Types`)))
    (`PrimitiveComponent.SetSimulatePhysics` _staticmesh true)
    (`KismetSystemLibrary.PrintString` "Spawned")
    (`KismetSystemLibrary.K2_SetTimerDelegate` (`|CreateDelegate` :!event `Drop`) (`KismetMathLibrary.RandomFloatInRange` 1.0 4.0))))

(event `/Game/Blueprints/BI_Signal.Enable/Disable`
  (params (Enabled :type Boolean))
  (set `self.IsOn` Enabled)
  (`self.Drop`))

(fn `UserConstructionScript`)