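; BP_Handle is an interactable gramophone crank that starts the record spinning and music playing.
; Each tick the actor snaps to a tagged static mesh found on the gramophone at BeginPlay.
; Interact runs once, playing a crank sound and Timeline rotation, then scratch audio, gated record spin and delayed music.
; HighlightEffect toggles the handle's custom depth until interaction closes its gate.
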(event `self.ReceiveBeginPlay`
  (bind _tags (`/Game/Blueprints/BPL_VisibilityAndTagging.MakeTags` (`|MakeArray` "NewEnumerator2" :!type "/Game/Blueprints/ENUM_Tags Enum")))
  (set `self.Qwob` (`|GetArrayItem` (`self.GetComponentsByTag` (`self.Grammaphone`) "/Script/Engine.StaticMeshComponent" (`|GetArrayItem` _tags))))
  (bind _tags_2 (`/Game/Blueprints/BPL_VisibilityAndTagging.MakeTags` (`|MakeArray` "NewEnumerator5" :!type "/Game/Blueprints/ENUM_Tags Enum")))
  (set `ActorComponent.ComponentTags` _tags_2 (`self.Collider`)))

(event `self.ReceiveTick`
  (params (DeltaSeconds :type "Float (single-precision)"))
  (bind (_returnvalue_location _returnvalue_rotation) (`KismetMathLibrary.BreakTransform` (`SceneComponent.K2_GetComponentToWorld` (`self.Qwob`))))
  (`self.K2_SetActorLocationAndRotation` _returnvalue_location _returnvalue_rotation false true)
  (`/Engine/EditorBlueprintResources/StandardMacros.Gate` true :!label _label
    (:`Exit`
      (`SceneComponent.K2_AddRelativeRotation` (`self.Record`) (`KismetMathLibrary.MakeRotator` 0.0 0.0 2.0) false true))))

(event `/Game/Blueprints/BI_ObjectFunctionality.Interact`
  (params (WasGrabbing :type Boolean))
  (`/Engine/EditorBlueprintResources/StandardMacros.DoOnce` false
    (:`Completed`
      (`|ExecutionSequence`
        (:`then_0`
          (`PrimitiveComponent.SetRenderCustomDepth` (`self.Handle`) false)
          (`GameplayStatics.PlaySoundAtLocation` "/Game/_Sound/SFX/GrammaphoneCrank.GrammaphoneCrank" (`self.K2_GetActorLocation`) (struct) 0.2 1.0 0.0 "/Game/FPSPuzzleSP/Blueprints/Components/SoundAttenuation.SoundAttenuation" null null null)
          (bind (_direction _newtrack_0) (`Timeline|Timeline`)
            (:`Update`
              (`SceneComponent.K2_SetRelativeRotation` (`self.Handle`) (`KismetMathLibrary.MakeRotator` _newtrack_0) false false))
            (:`Finished`
              (`AudioComponent.Play` (`self.Scratch`) 0.0)
              (`|ExecutionSequence`
                (:`then_0`
                  (goto _label :!via `Open`))
                (:`then_1`
                  (`KismetSystemLibrary.Delay` 1.0)
                  (`AudioComponent.Play` (`self.Music`) 0.0))))))
        (:`then_1`
          (goto _label_2 :!via `Close`))))))

(event `/Game/Blueprints/BI_ObjectFunctionality.HighlightEffect`
  (params (IsOn :type Boolean))
  (`/Engine/EditorBlueprintResources/StandardMacros.Gate` false :!label _label_2
    (:`Exit`
      (`PrimitiveComponent.SetRenderCustomDepth` (`self.Handle`) IsOn))))

(fn `UserConstructionScript`)