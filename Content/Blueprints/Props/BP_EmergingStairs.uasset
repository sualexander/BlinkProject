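; Stairs prop that emerges or retracts on an On/Off Turn signal, using a Level 3 exit stairs material.
; BeginPlay creates a dynamic material instance, and the Increment timeline drives its Amount parameter, playing forward for On and reversing for Off.
; When the timeline finishes, mesh collision is enabled after On and disabled after Off.
; The IsOn flag is inverted relative to its name: false after On, true after Off.
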(event `self.ReceiveBeginPlay`
  (bind _returnvalue (`PrimitiveComponent.CreateDynamicMaterialInstance` (`self.StaticMesh`) 0 "/Game/Materials/Area1/MI_Level3ExitStairs.MI_Level3ExitStairs" "None"))
  (set `self.Material` _returnvalue))

(event `/Game/Blueprints/BI_Signal.Turn`
  (params (Signal :type "/Game/FPSPuzzleSP/Blueprints/Components/Enum_Signal Enum" :default "NewEnumerator0"))
  (bind _staticmesh (`self.StaticMesh`))
  (switch `/Game/FPSPuzzleSP/Blueprints/Components/Enum_Signal` Signal
    (:`NewEnumerator0`
      (set `self.IsOn` false)
      (bind (_direction _alpha) (`Timeline|Increment` :!label _label)
        (:`Update`
          (`MaterialInstanceDynamic.SetScalarParameterValue` (`self.Material`) "Amount" _alpha))
        (:`Finished`
          (if (`self.IsOn`)
            (`PrimitiveComponent.SetCollisionEnabled` _staticmesh "NoCollision")
            (else
              (`PrimitiveComponent.SetCollisionEnabled` _staticmesh "QueryAndPhysics"))))))
    (:`NewEnumerator1`
      (set `self.IsOn` true)
      (goto _label :!via `Reverse`))))

(fn `UserConstructionScript`)