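; BP_CloudSwitcher is a prop that swaps the sky's volumetric cloud formation whenever its Cube goes out of view after being seen.
; BeginPlay caches the Cube's unique scaled mesh vertices, which Tick uses for visibility checks.
; On each visible-to-hidden transition, it destroys and respawns the VolumetricCloud and a cloud mask object, cycling mask positions through the Positions array.
; Enable/Disable toggles this behavior through actor tick.
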(event `self.ReceiveBeginPlay`
  (bind _cube (`self.Cube`))
  (bind _vertices (`KismetProceduralMeshLibrary.GetSectionFromStaticMesh` (`StaticMeshComponent.StaticMesh` _cube)))
  (for _array_element _vertices
    (`KismetArrayLibrary.Array_AddUnique` (`self.Verts`) (* _array_element (`SceneComponent.K2_GetComponentScale` _cube))))
  (bind _tags (`/Game/Blueprints/BPL_VisibilityAndTagging.MakeTags` (`|MakeArray` "NewEnumerator0" :!type "/Game/Blueprints/ENUM_Tags Enum")))
  (set `ActorComponent.ComponentTags` _tags (`self.Cube`)))

(event `/Game/Blueprints/BI_Signal.Enable/Disable`
  (params (Enabled :type Boolean))
  (`self.SetActorTickEnabled` Enabled))

(event `self.ReceiveTick`
  (params (DeltaSeconds :type "Float (single-precision)"))
  (bind _positions (`self.Positions`))
  (bind _isvisible (`/Game/Blueprints/BPL_VisibilityAndTagging.Is Component Visible` (`self.Verts`) (`self.Cube`)))
  (if _isvisible
    (set `self.HasUpdated` true)
    (elif (`self.HasUpdated`)
      (set `self.HasUpdated` false)
      (bind _returnvalue (`GameplayStatics.GetActorOfClass` "/Script/Engine.VolumetricCloud"))
      (`self.K2_DestroyActor` _returnvalue)
      (`self.K2_DestroyActor` (`self.Cloud`))
      (bind _returnvalue_2 (`|SpawnActorFromClass` "/Script/Engine.VolumetricCloud" (`KismetMathLibrary.MakeTransform` (0.0 0.0 0.0)) "AlwaysSpawn" "OverrideRootScale" null null))
      (bind _volumetriccloudcomponent (`VolumetricCloud.VolumetricCloudComponent` _returnvalue_2))
      (`VolumetricCloudComponent.SetMaterial` _volumetriccloudcomponent "/Volumetrics/Content/Sky/Materials/M_VolumetricCloud_02_Profiles_Soft.M_VolumetricCloud_02_Profiles_Soft")
      (`VolumetricCloudComponent.SetLayerBottomAltitude` _volumetriccloudcomponent 2.0)
      (bind _result (`/Engine/EditorBlueprintResources/StandardMacros.IncrementInt` (`self.Index`))
        (:`  `
          (bind _returnvalue_3 (`|SpawnActorFromClass` "/Volumetrics/Tools/CloudCompositing/Blueprints/BP_CloudMask_Object.BP_CloudMask_Object_C" (`KismetMathLibrary.MakeTransform` (`|GetArrayItem` _positions (mod _result (`KismetArrayLibrary.Array_Length` _positions))) (struct) (10.0 10.0 10.0)) "AlwaysSpawn" "OverrideRootScale" null null))
          (set `self.Cloud` _returnvalue_3)
          (set `/Volumetrics/Tools/CloudCompositing/Blueprints/BP_CloudMask_Object.Noise Settings` (make `/Volumetrics/Tools/CloudCompositing/Blueprints/Structs/CloudNoiseSettings` 0.5 0.6 3.0) _returnvalue_3))))))

(fn `UserConstructionScript`)