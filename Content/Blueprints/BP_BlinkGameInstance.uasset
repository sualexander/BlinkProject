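; Game instance for Blink that manages background music persisting across level transitions.
; PlayMusic calls the Play event, which fades out and destroys the current track after a delay, then creates and fades in the new 2D sound.
; SetLowPass sets the current track's low-pass frequency and prints a debug string.
; SelectLevel is an empty event; its level-opening and streaming logic is disconnected, as is older music code in PlayMusic.
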(event `Play`
  (params (Track :type "SoundBase Object Reference") (Volume :type "Float (single-precision)"))
  (bind _currentmusic (`self.CurrentMusic`)
    (:`then`
      (`AudioComponent.FadeOut` _currentmusic 4.0 0.0 "Linear")
      (`KismetSystemLibrary.Delay` 4.0)
      (`ActorComponent.K2_DestroyComponent` _currentmusic))
    (:`else`
      _))
  (bind _returnvalue (`GameplayStatics.CreateSound2D` Track Volume 1.0 0.0 null true))
  (set `self.CurrentMusic` _returnvalue)
  (`AudioComponent.FadeIn` _returnvalue 2.0 1.0 0.0 "Linear"))

(event `SelectLevel`
  (params (Level :type "/Game/Blueprints/ENUM_Levels Enum" :default "NewEnumerator2")))

(fn `PlayMusic`
  (params (Track :type "SoundBase Object Reference") (Volume :type "Float (single-precision)"))
  (`self.Play` Track Volume))

(fn `SetLowPass`
  (params (InLowPassFilterFrequency :type "Float (single-precision)"))
  (`AudioComponent.SetLowPassFilterFrequency` (`self.CurrentMusic`) InLowPassFilterFrequency)
  (`KismetSystemLibrary.PrintString` "SET LOW PASS"))