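; Blueprint function library that tests whether a component is visible to player 0, given a list of its local vertices.
; Vertices are moved to world space by rotation and location (no scale), then pass if any projects inside the viewport.
; Multi line traces against WorldStatic then run from the camera to each vertex.
; Hitting the component means visible; "Marker"-tagged components are seen through, while other hits block that ray.
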(fn `Is Component in FOV`
  (params (Vertices :type "Array of Vector Structure"))
  (returns (IsInFOV :type Boolean))
  (bind (_returnvalue_x _returnvalue_y) (`KismetMathLibrary.BreakVector2D` (`WidgetLayoutLibrary.GetViewportSize` null)))
  (for _array_element Vertices
    (bind _screenlocation (`PlayerController.ProjectWorldLocationToScreen` (`GameplayStatics.GetPlayerController` null) _array_element false))
    (if (and (> (`KismetMathLibrary.BreakVector2D` _screenlocation) 0.0) (< (`KismetMathLibrary.BreakVector2D` _screenlocation) _returnvalue_x) (> (`.Y` (`KismetMathLibrary.BreakVector2D` _screenlocation)) 0.0) (< (`.Y` (`KismetMathLibrary.BreakVector2D` _screenlocation)) _returnvalue_y))
      (return true)))
  (return false))

(fn `Is Component Visible`
  (params (Vertices :type "Array of Vector Structure") (Component :type "StaticMeshComponent Object Reference"))
  (returns (IsVisible :type Boolean))
  (locals (WorldPositions :type "Array of Vector Structure"))
  (bind _worldpositions (`local.WorldPositions`))
  (for _array_element Vertices
    (`KismetArrayLibrary.Array_Add` _worldpositions (+ (`KismetMathLibrary.GreaterGreater_VectorRotator` _array_element (`SceneComponent.K2_GetComponentRotation` Component)) (`SceneComponent.K2_GetComponentLocation` Component))))
  (bind _isinfov (`self.Is Component in FOV` _worldpositions))
  (if _isinfov
    (for _array_element_2 _worldpositions
      (bind _outhits (`KismetSystemLibrary.LineTraceMultiForObjects` :`Start` (`Actor.K2_GetActorLocation` (`GameplayStatics.GetPlayerCameraManager` null)) :`End` _array_element_2 :`ObjectTypes` (`|MakeArray` "ObjectTypeQuery1" :!type "EObjectTypeQuery Enum") :`bIgnoreSelf` false))
      (if (> (`KismetArrayLibrary.Array_Length` _outhits) 0)
        (for _array_element_3 _outhits
          (bind (_bblockinghit _binitialoverlap _time _distance _location _impactpoint _normal _impactnormal _physmat _hitactor _hitcomponent) (`GameplayStatics.BreakHitResult` _array_element_3))
          (if (== (`local.Component`) _hitcomponent)
            (return true)
            (elif (not (`ActorComponent.ComponentHasTag` _hitcomponent "Marker"))
              (break))))))
    (return false)
    (else
      (return false))))