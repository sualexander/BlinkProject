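; BP_SpringArmComponent is a physics grab component on BP_MainPlayer that holds a grabbed component at a point in front of itself.
; Attaching stores the component's gravity and damping, overrides them and enables tick; detaching restores them, adds a vertical push and stops ticking.
; Each tick applies a distance-scaled acceleration toward the hold point, or forces the player to ungrab when the object is too far away.
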(event `self.ReceiveBeginPlay`
  ;[0 0 0] BeginPlay: Get reference to player
  (bind _asbp_main_player (cast `/Game/Blueprints/BP_MainPlayer` (`self.GetOwner`))
    (:`then`
      (set `self.PlayerREF` _asbp_main_player))
    (:`CastFailed`
      (`KismetSystemLibrary.PrintString` "SpringArmComponent Attached To Wrong Actor!"))))

(event `AttachComponent`
  (params (NewAttached :type "PrimitiveComponent Object Reference"))
  ;[0 0 0] Ongrab: Enable event tick and set parameters
  (`self.AttachedComponent`
    (:`then`
      (`self.DetachComponent`))
    (:`else`
      _))
  (`/Engine/EditorBlueprintResources/StandardMacros.IsValid` NewAttached
    (:`Is Valid`
      (bind _output_get (set `self.AttachedComponent` NewAttached))
      (`self.SetComponentTickEnabled` true)
      (`self.Set Paramters for Grabbed` _output_get))))

(event `DetachComponent`
  ;[0 0 0] Ungrab: Disable event tick and reset parameters
  (bind _attachedcomponent (`self.AttachedComponent`)
    (:`then`
      (`self.ResetToOriginalParameters` _attachedcomponent)
      (`PrimitiveComponent.AddForce` _attachedcomponent (`KismetMathLibrary.MakeVector` 0.0 0.0 (`self.GravityPush`)) "None" true)
      (set `self.AttachedComponent` null)
      (`self.SetComponentTickEnabled` false))
    (:`else`)))

(event `self.ReceiveTick`
  (params (DeltaSeconds :type "Float (single-precision)"))
  ;[0 0 0] EventTick: Update grabbed component location when grabbing
  (bind _attachedcomponent (`self.AttachedComponent`)
    (:`then`
      (`self.PushComponentToGrabLocation` _attachedcomponent))
    (:`else`)))

(fn `PushComponentToGrabLocation`
  (params (AttachedComponent :type "SceneComponent Object Reference"))
  (bind _returnvalue (`self.K2_GetComponentLocation` AttachedComponent))
  ;[0 0 0] Add force towards grab location, if grabbed component is too far away (ex: stuck behind wall) force ungrab
  (bind _output_get (set `self.TargetLocation` (+ (`self.K2_GetComponentLocation`) (* (`self.GetForwardVector`) (`self.GrabLength`)) (`self.GrabLocationOffset`))))
  (if (> (`KismetMathLibrary.VSize` (- _returnvalue (`Actor.K2_GetActorLocation` (`self.PlayerREF`)))) (`self.MaxDistance`))
    (`/Game/Blueprints/BP_MainPlayer.ForcedUngrab` (`self.PlayerREF`))
    (`KismetSystemLibrary.PrintString` "UNGRABED: Too far away from object")
    (else
      (bind _returnvalue_2 (- _output_get _returnvalue))
      (`PrimitiveComponent.AddForce` (`self.AttachedComponent`) (* (`KismetMathLibrary.Normal` _returnvalue_2) (`KismetMathLibrary.MapRangeClamped` (`KismetMathLibrary.VSize` _returnvalue_2) (`self.MinStrengthDistance`) (`self.MaxStrengthDistance`) (`self.MinStrength`) (`self.MaxStrength`))) "None" true))))

(fn `ResetToOriginalParameters`
  (params (AttachedComponent :type "PrimitiveComponent Object Reference"))
  ;[0 0 0] Reset parameters:
  (`PrimitiveComponent.SetLinearDamping` AttachedComponent (`self.OriginalLinearDamping`))
  (`PrimitiveComponent.SetAngularDamping` AttachedComponent (`self.OriginalAngularDamping`))
  (`PrimitiveComponent.SetEnableGravity` AttachedComponent (`self.OriginalGravity`)))

(fn `Set Paramters for Grabbed`
  (params (AttachedComponent :type "PrimitiveComponent Object Reference"))
  ;[0 0 0] Disable gravity, set damping values, store original physics parameters
  (set `self.OriginalGravity` (`PrimitiveComponent.IsGravityEnabled` AttachedComponent))
  (set `self.OriginalLinearDamping` (`PrimitiveComponent.GetLinearDamping` AttachedComponent))
  (set `self.OriginalAngularDamping` (`PrimitiveComponent.GetAngularDamping` AttachedComponent))
  (`PrimitiveComponent.SetSimulatePhysics` AttachedComponent true)
  (`PrimitiveComponent.SetEnableGravity` AttachedComponent false)
  (`PrimitiveComponent.SetLinearDamping` AttachedComponent (`self.LinearDamping`))
  (`PrimitiveComponent.SetAngularDamping` AttachedComponent (`self.AngularDamping`)))