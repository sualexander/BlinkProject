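; Blueprint function library that tests whether a component is visible to player 0 and provides enum-based tag helpers.
; Visibility rotates and offsets the supplied vertices to world space, ignoring scale, and requires one to project inside the viewport.
; It then multi-traces WorldStatic from the camera to each vertex, looking past specifically tagged components until it hits the target or another blocker.
; The tag helpers convert enum values to names to build and query tag arrays.
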(fn `CheckIfAnyTags`
  (params (CheckedTags :type "Array of /Game/Blueprints/E_Tags Enum") (Tags :type "Array of Name"))
  (returns (HasTag :type Boolean))
  (for _array_element CheckedTags
    (for _array_element_2 Tags
      (if (== _array_element_2 (`|GetEnumeratorName` _array_element))
        (return true))))
  (return false))

(fn `CheckTag`
  (params (CheckedTag :type "/Game/Blueprints/E_Tags Enum" :default "NewEnumerator0") (Tags :type "Array of Name"))
  (returns (HasTag :type Boolean))
  (for _array_element Tags
    (if (== _array_element (`|GetEnumeratorName` CheckedTag))
      (return true)))
  (return false))

(fn `Is Component in FOV`
  (params (Vertices :type "Array of Vector Structure"))
  (returns (IsInFOV :type Boolean))
  (bind (_returnvalue_x _returnvalue_y) (`KismetMathLibrary.BreakVector2D` (`WidgetLayoutLibrary.GetViewportSize` null)))
  (for _array_element Vertices
    (bind _screenlocation (`PlayerController.ProjectWorldLocationToScreen` (`GameplayStatics.GetPlayerController` null) _array_element false))
    (if (and (> (`KismetMathLibrary.BreakVector2D` _screenlocation) 0.0) (< (`KismetMathLibrary.BreakVector2D` _screenlocation) _returnvalue_x) (> (`.Y` (`KismetMathLibrary.BreakVector2D` _screenlocation)) 0.0) (< (`.Y` (`KismetMathLibrary.BreakVector2D` _screenlocation)) _returnvalue_y))
      (return true)))
  (return false))

(fn `Is Component Visible`
  (params (Vertices :type "Array of Vector Structure") (Component :type "StaticMeshComponent Object Reference"))
  (returns (IsVisible :type Boolean))
  (locals (WorldPositions :type "Array of Vector Structure"))
  (bind _worldpositions (`local.WorldPositions`))
  (for _array_element Vertices
    (`KismetArrayLibrary.Array_Add` _worldpositions (+ (`KismetMathLibrary.GreaterGreater_VectorRotator` _array_element (`SceneComponent.K2_GetComponentRotation` Component)) (`SceneComponent.K2_GetComponentLocation` Component))))
  (bind _isinfov (`self.Is Component in FOV` _worldpositions))
  (if _isinfov
    (for _array_element_2 _worldpositions
      (bind _outhits (`KismetSystemLibrary.LineTraceMultiForObjects` :`Start` (`Actor.K2_GetActorLocation` (`GameplayStatics.GetPlayerCameraManager` null)) :`End` _array_element_2 :`ObjectTypes` (`|MakeArray` "ObjectTypeQuery1" :!type "EObjectTypeQuery Enum") :`bIgnoreSelf` false))
      (if (> (`KismetArrayLibrary.Array_Length` _outhits) 0)
        (for _array_element_3 _outhits
          (bind (_bblockinghit _binitialoverlap _time _distance _location _impactpoint _normal _impactnormal _physmat _hitactor _hitcomponent) (`GameplayStatics.BreakHitResult` _array_element_3))
          (if (== (`local.Component`) _hitcomponent)
            (return true)
            (else
              (bind _hastag (`self.CheckIfAnyTags` (`|MakeArray` "NewEnumerator0" "NewEnumerator1" :!type "/Game/Blueprints/E_Tags Enum") (`ActorComponent.ComponentTags` _hitcomponent)))
              (if (not _hastag)
                (break)))))))
    (return false)
    (else
      (return false))))

(fn `MakeTags`
  (params (TagsToSet :type "Array of /Game/Blueprints/E_Tags Enum"))
  (returns (Tags :type "Array of Name"))
  (locals (FinalTags :type "Array of Name"))
  (bind _finaltags (`local.FinalTags`))
  (for _array_element TagsToSet
    (`KismetArrayLibrary.Array_AddUnique` _finaltags (`|GetEnumeratorName` _array_element)))
  (return _finaltags))