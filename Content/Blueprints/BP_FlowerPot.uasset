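; BP_FlowerPot is a flowerpot actor with a grab component, apparently a work-in-progress grabbable physics prop.
; On BeginPlay it caches the player, binds UpdateGrab to the grab component's attach event and enables physics after a short delay.
; UpdateGrab only checks the grabbing state, while Tick nudges the pot along world X every frame.
; Camera attach, detach and Chaos break logic is present but disconnected.
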(event `self.ReceiveBeginPlay`
  (add `/Game/Blueprints/BP_GrabComponent.AttachComponents` (`self.BP_GrabComponent`) (delegate `UpdateGrab`))
  (bind _asbp_main_player (cast `/Game/Blueprints/BP_MainPlayer` (`GameplayStatics.GetPlayerPawn` 0)))
  (set `self.PlayerREF` _asbp_main_player)
  (`KismetSystemLibrary.Delay` 1.0)
  (`PrimitiveComponent.SetSimulatePhysics` (`self.Flowerpot`) true)
  (`KismetSystemLibrary.PrintString` "Let Go"))

(event `UpdateGrab`
  (if (`/Game/Blueprints/BP_GrabComponent.Is Grabbing` (`self.BP_GrabComponent`))
    _))

(event `self.ReceiveTick`
  (params (DeltaSeconds :type "Float (single-precision)"))
  (`SceneComponent.K2_AddWorldOffset` (`self.Flowerpot`) (1.0 0.0 0.0) false false))

(fn `UserConstructionScript`)