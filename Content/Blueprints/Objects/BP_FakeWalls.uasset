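; BP_FakeWalls is an actor that teleports its Qwob to a randomly picked marker the player cannot see.
; BeginPlay hides components tagged Marker and caches the first marker's unique, scaled mesh vertices for visibility tests.
; A one-time box overlap enables Tick, which tests markers in random order until one is unseen.
; It then moves Qwob there, stops ticking and calls FinalAction, an empty event.
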(event `self.ReceiveBeginPlay`
  ;[0 0 0] BeginPlay: Initialize Markers and Qwob
  (`|ExecutionSequence`
    (:`then_0`
      (bind _output_get (set `self.Markers` (`self.GetComponentsByTag` "/Script/Engine.StaticMeshComponent" "Marker")))
      (set `self.NumMarkers` (`KismetArrayLibrary.Array_Length` _output_get))
      (set `self.CurrentMarker` -1)
      (`self.GetVertices` _output_get))
    (:`then_1`
      (for _array_element (`self.Markers`)
        (`SceneComponent.SetHiddenInGame` _array_element true false)))))

(event `self.ReceiveTick`
  (params (DeltaSeconds :type "Float (single-precision)"))
  (bind (_index _found) (`self.SearchMarkers`))
  (if _found
    (`/Engine/EditorBlueprintResources/StandardMacros.DoOnce` false
      (:`Completed`
        (`self.UpdateQWOB` _index)
        (`self.SetActorTickEnabled` false)
        (`self.FinalAction`)))))

(event `FinalAction`)

(event `self.Box.OnComponentBeginOverlap`
  (params (OverlappedComponent :type "PrimitiveComponent Object Reference") (OtherActor :type "Actor Object Reference") (OtherComp :type "PrimitiveComponent Object Reference") (OtherBodyIndex :type Integer) (bFromSweep :type Boolean) (SweepResult :type "HitResult Structure (by ref)"))
  (`/Engine/EditorBlueprintResources/StandardMacros.DoOnce` false
    (:`Completed`
      (`self.SetActorTickEnabled` true))))

(fn `GenerateIndices`
  (params (NumIndices :type Integer))
  (bind _indices (`self.Indices`))
  ;[0 0 0] Make integer array of element index
  (`KismetArrayLibrary.Array_Clear` _indices)
  (for _index (range NumIndices)
    (`KismetArrayLibrary.Array_Add` _indices _index))
  (`KismetArrayLibrary.Array_RemoveItem` _indices (`self.CurrentMarker`))
  (return))

(fn `GetVertices`
  (params (Array :type "Array of StaticMeshComponent Object Reference"))
  (bind _output (`|GetArrayItem` Array))
  ;[0 0 0] Stores vertices of mesh, removes duplicates
  (bind _vertices (`KismetProceduralMeshLibrary.GetSectionFromStaticMesh` (`StaticMeshComponent.StaticMesh` _output)))
  (for _array_element _vertices
    (`KismetArrayLibrary.Array_AddUnique` (`self.Vertices`) (* _array_element (`SceneComponent.K2_GetComponentScale` _output)))))

(fn `IsVisible`
  (returns (IsVisible :type Boolean))
  (bind _isvisible (`self.ToObjectRaycast`))
  (if _isvisible
    (return true)
    (else
      (return false))))

(fn `SearchMarkers`
  (returns (Index :type Integer) (Found :type Boolean))
  (locals (RandomIndex :type Integer :default 0))
  (bind _indices (`self.Indices`))
  (bind _returnvalue (`KismetArrayLibrary.Array_Length` _indices))
  ;[0 0 0] Search through all markers, return any not visible if any
  (`self.GenerateIndices` (`self.NumMarkers`))
  (while (> _returnvalue 0)
    (bind _output_get (set `local.RandomIndex` (`KismetMathLibrary.RandomInteger` _returnvalue)))
    (bind _output (`|GetArrayItem` _indices _output_get))
    (bind _isvisible (`/Game/Blueprints/BPL_VisibilityAndTagging.Is Component Visible` (`self.Vertices`) (`|GetArrayItem` (`self.Markers`) _output)))
    (if _isvisible
      (`KismetArrayLibrary.Array_RemoveItem` _indices _output)
      (else
        (return _output true))))
  (return 0 false))

(fn `ToObjectRaycast`
  (returns (IsVisible :type Boolean))
  ;[0 0 0] Calls visibility function on current marker
  (bind _isvisible (`/Game/Blueprints/BPL_VisibilityAndTagging.Is Component Visible` (`self.Vertices`) (`|GetArrayItem` (`self.Markers`) (`self.CurrentMarker`))))
  (return _isvisible))

(fn `UpdateQWOB`
  (params (Marker :type Integer))
  ;[0 0 0] Teleports Qwob to selected marker
  (bind _output_get (set `self.CurrentMarker` Marker))
  (`SceneComponent.K2_SetWorldLocation` (`self.QWOB`) (`SceneComponent.K2_GetComponentLocation` (`|GetArrayItem` (`self.Markers`) _output_get)) false true))

(fn `UserConstructionScript`)