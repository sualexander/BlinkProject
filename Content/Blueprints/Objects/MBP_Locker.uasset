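; Switchable locker object that sends lock messages to MBI_ObjectFunctionality actors inside its collider.
; Overlaps send lock or unlock regardless of on/off state and add actors to LockedActors, which never removes them.
; On/Off signals re-send lock or unlock to that whole list, toggling the spotlight, sound and tick-driven light rotation.
; When initially on, it also scans for actors already overlapping at BeginPlay.
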(event `self.ReceiveBeginPlay`
  (if (`self.IsInitiallyOn`)
    (`self.Activate`)
    (bind _outactors (`GameplayStatics.GetAllActorsWithInterface` "/Game/Blueprints/MBI_ObjectFunctionality.MBI_ObjectFunctionality_C"))
    (for _array_element _outactors
      (if (`self.IsOverlappingActor` _array_element self)
        (message `/Game/Blueprints/MBI_ObjectFunctionality.UpdateLock` _array_element true)
        (`KismetArrayLibrary.Array_AddUnique` (`self.LockedActors`) _array_element)))
    (else
      (`self.Deactivate`))))

(event `self.ReceiveTick`
  (params (DeltaSeconds :type "Float (single-precision)"))
  (`SceneComponent.K2_AddWorldRotation` (`self.LightBase`) (struct :`Yaw` 0.5) false false))

(event `self.Collider.OnComponentBeginOverlap`
  (params (OverlappedComponent :type "PrimitiveComponent Object Reference") (OtherActor :type "Actor Object Reference") (OtherComp :type "PrimitiveComponent Object Reference") (OtherBodyIndex :type Integer) (bFromSweep :type Boolean) (SweepResult :type "HitResult Structure (by ref)"))
  (if (`KismetSystemLibrary.DoesImplementInterface` OtherActor "/Game/Blueprints/MBI_ObjectFunctionality.MBI_ObjectFunctionality_C")
    (message `/Game/Blueprints/MBI_ObjectFunctionality.UpdateLock` OtherActor true)
    (`KismetArrayLibrary.Array_AddUnique` (`self.LockedActors`) OtherActor)))

(event `self.Collider.OnComponentEndOverlap`
  (params (OverlappedComponent :type "PrimitiveComponent Object Reference") (OtherActor :type "Actor Object Reference") (OtherComp :type "PrimitiveComponent Object Reference") (OtherBodyIndex :type Integer))
  (if (`KismetSystemLibrary.DoesImplementInterface` OtherActor "/Game/Blueprints/MBI_ObjectFunctionality.MBI_ObjectFunctionality_C")
    (for _array_element (`self.LockedActors`)
      (if (== _array_element OtherActor)
        (message `/Game/Blueprints/MBI_ObjectFunctionality.UpdateLock` OtherActor false)
        (break)))))

(event `Activate`
  (for _array_element (`self.LockedActors`)
    (message `/Game/Blueprints/MBI_ObjectFunctionality.UpdateLock` _array_element true))
  (`SceneComponent.SetVisibility` (`self.SpotLight`) true false)
  (`GameplayStatics.PlaySoundAtLocation` "/Engine/VREditor/Sounds/UI/Dockable_Window_Open.Dockable_Window_Open" (`SceneComponent.K2_GetComponentLocation` (`self.Collider`)) (struct) 2.0 1.0 0.0 "/Game/FPSPuzzleSP/Blueprints/Components/SoundAttenuation.SoundAttenuation" null null null)
  (`self.SetActorTickEnabled` true))

(event `/Game/Blueprints/BI_Signal.Update`
  (params (Signal :type "/Game/FPSPuzzleSP/Blueprints/Components/Enum_Signal Enum" :default "NewEnumerator0"))
  (switch `/Game/FPSPuzzleSP/Blueprints/Components/Enum_Signal` Signal
    (:`NewEnumerator0`
      (`self.Activate`))
    (:`NewEnumerator1`
      (`self.Deactivate`))))

(event `Deactivate`
  (for _array_element (`self.LockedActors`)
    (message `/Game/Blueprints/MBI_ObjectFunctionality.UpdateLock` _array_element false))
  (`SceneComponent.SetVisibility` (`self.SpotLight`) false false)
  (`GameplayStatics.PlaySoundAtLocation` "/Engine/VREditor/Sounds/UI/Dockable_Window_Close.Dockable_Window_Close" (`SceneComponent.K2_GetComponentLocation` (`self.Collider`)) (struct) 2.0 1.0 0.0 "/Game/FPSPuzzleSP/Blueprints/Components/SoundAttenuation.SoundAttenuation" null null null)
  (`self.SetActorTickEnabled` false))

(fn `UserConstructionScript`)