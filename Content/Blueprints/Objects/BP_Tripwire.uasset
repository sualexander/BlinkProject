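; BP_Tripwire is a box trigger that signals linked objects as the player enters or leaves it.
; Overlap begin and end send opposite UpdateMessage states to each target in Outputs, with a per-entry InvertSignal flag swapping them.
; Targets in OutputsEnable get EnableDisableMessage, receiving InvertSignal on entry and its negation on exit.
; Actors other than BP_MainPlayer are ignored.
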(event `self.Box.OnComponentBeginOverlap`
  (params (OverlappedComponent :type "PrimitiveComponent Object Reference") (OtherActor :type "Actor Object Reference") (OtherComp :type "PrimitiveComponent Object Reference") (OtherBodyIndex :type Integer) (bFromSweep :type Boolean) (SweepResult :type "HitResult Structure (by ref)"))
  (cast `/Game/Blueprints/BP_MainPlayer` OtherActor)
  (for _array_element (`self.Outputs`)
    (message `/Game/Blueprints/BI_Signal.Update` (break `/Game/Blueprints/STRUCT_Signals` _array_element) (select `bool` (`.InvertSignal_5_DAF274A9474CC75ECB928ABBDE614AD0` (break `/Game/Blueprints/STRUCT_Signals` _array_element)) :`false` "NewEnumerator0" :`true` "NewEnumerator1" :!type "/Game/FPSPuzzleSP/Blueprints/Components/Enum_Signal Enum")))
  (for _array_element_2 (`self.OutputsEnable`)
    (message `/Game/Blueprints/BI_Signal.Enable/Disable` (break `/Game/Blueprints/STRUCT_Signals` _array_element_2) (`.InvertSignal_5_DAF274A9474CC75ECB928ABBDE614AD0` (break `/Game/Blueprints/STRUCT_Signals` _array_element_2)))))

(event `self.Box.OnComponentEndOverlap`
  (params (OverlappedComponent :type "PrimitiveComponent Object Reference") (OtherActor :type "Actor Object Reference") (OtherComp :type "PrimitiveComponent Object Reference") (OtherBodyIndex :type Integer))
  (cast `/Game/Blueprints/BP_MainPlayer` OtherActor)
  (for _array_element (`self.Outputs`)
    (message `/Game/Blueprints/BI_Signal.Update` (break `/Game/Blueprints/STRUCT_Signals` _array_element) (select `bool` (`.InvertSignal_5_DAF274A9474CC75ECB928ABBDE614AD0` (break `/Game/Blueprints/STRUCT_Signals` _array_element)) :`false` "NewEnumerator1" :`true` "NewEnumerator0" :!type "/Game/FPSPuzzleSP/Blueprints/Components/Enum_Signal Enum")))
  (for _array_element_2 (`self.OutputsEnable`)
    (message `/Game/Blueprints/BI_Signal.Enable/Disable` (break `/Game/Blueprints/STRUCT_Signals` _array_element_2) (not (`.InvertSignal_5_DAF274A9474CC75ECB928ABBDE614AD0` (break `/Game/Blueprints/STRUCT_Signals` _array_element_2))))))

(fn `UserConstructionScript`)