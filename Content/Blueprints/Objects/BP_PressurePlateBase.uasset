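; Base pressure plate that signals linked output targets when a Qwob's tagged component enters or leaves its trigger.
; Overlap events track the current Qwob and call overridable animation events, which by default send activation or deactivation messages to each output, optionally inverted.
; Shortly after BeginPlay it checks existing overlaps and activates directly if one qualifies.
; Empty AfterSignalOn and AfterSignalOff events act as hooks following each signal.
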(event `self.ReceiveBeginPlay`
  (bind _asbp_main_player (cast `/Game/Blueprints/BP_MainPlayer` (`GameplayStatics.GetPlayerCharacter` 0)))
  (set `self.PlayerREF` _asbp_main_player)
  (`KismetSystemLibrary.Delay` 0.2)
  (bind _hasinitialoverlap (`self.CheckInitialOverlaps`))
  (if _hasinitialoverlap
    (`self.SendActivation`)))

(event `self.Trigger.OnComponentBeginOverlap`
  (params (OverlappedComponent :type "PrimitiveComponent Object Reference") (OtherActor :type "Actor Object Reference") (OtherComp :type "PrimitiveComponent Object Reference") (OtherBodyIndex :type Integer) (bFromSweep :type Boolean) (SweepResult :type "HitResult Structure (by ref)"))
  (if (not (`self.IsActive`))
    (bind _hastag (`/Game/Blueprints/BPL_VisibilityAndTagging.CheckTag` "NewEnumerator3" (`ActorComponent.ComponentTags` OtherComp)))
    (if _hastag
      (set `self.CurrentQwob` OtherActor)
      (`self.ActivateAnim` OtherComp))))

(event `SendActivation`
  (set `self.IsActive` true)
  (for _array_element (`self.Outputs`)
    (message `/Game/Blueprints/BI_Signal.Update` (break `/Game/Blueprints/STRUCT_Signals` _array_element) (select `bool` (`.InvertSignal_5_DAF274A9474CC75ECB928ABBDE614AD0` (break `/Game/Blueprints/STRUCT_Signals` _array_element)) :`false` "NewEnumerator0" :`true` "NewEnumerator1" :!type "/Game/FPSPuzzleSP/Blueprints/Components/Enum_Signal Enum")))
  (`self.AfterSignalOn`))

(event `self.Trigger.OnComponentEndOverlap`
  (params (OverlappedComponent :type "PrimitiveComponent Object Reference") (OtherActor :type "Actor Object Reference") (OtherComp :type "PrimitiveComponent Object Reference") (OtherBodyIndex :type Integer))
  (if (`self.IsActive`)
    (bind _hastag (`/Game/Blueprints/BPL_VisibilityAndTagging.CheckTag` "NewEnumerator3" (`ActorComponent.ComponentTags` OtherComp)))
    (if _hastag
      (`self.DeactivateAnim`)
      (set `self.CurrentQwob` null))))

(event `SendDeactivation`
  (set `self.IsActive` false)
  (for _array_element (`self.Outputs`)
    (message `/Game/Blueprints/BI_Signal.Update` (break `/Game/Blueprints/STRUCT_Signals` _array_element) (select `bool` (`.InvertSignal_5_DAF274A9474CC75ECB928ABBDE614AD0` (break `/Game/Blueprints/STRUCT_Signals` _array_element)) :`false` "NewEnumerator1" :`true` "NewEnumerator0" :!type "/Game/FPSPuzzleSP/Blueprints/Components/Enum_Signal Enum")))
  (`self.AfterSignalOff`))

(event `AfterSignalOn`)

(event `ActivateAnim`
  (params (QwobMarker :type "PrimitiveComponent Object Reference"))
  (`self.SendActivation`))

(event `AfterSignalOff`)

(event `DeactivateAnim`
  (`self.SendDeactivation`))

(fn `CheckInitialOverlaps`
  (returns (HasInitialOverlap :type Boolean))
  (for _array_element (`PrimitiveComponent.GetOverlappingComponents` (`self.Trigger`))
    (bind _hastag (`/Game/Blueprints/BPL_VisibilityAndTagging.CheckTag` "NewEnumerator3" (`ActorComponent.ComponentTags` _array_element)))
    (if _hastag
      (return true)))
  (return false))

(fn `UserConstructionScript`)