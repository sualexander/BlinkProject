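; BP_LightBreaker is an object that periodically switches lights off and on through the player character, with a breaker sound.
; On BeginPlay it caches BP_MainPlayer and starts a looping timer on a Test event.
; A FlipFlop in that event alternates between TurnOffLights and TurnOnLights, starting with off.
; Both pass the state to the player's UpdateLights and play the sound at the breaker's location.
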(event `self.ReceiveBeginPlay`
  (bind _asbp_main_player (cast `/Game/Blueprints/BP_MainPlayer` (`GameplayStatics.GetPlayerCharacter` 0)))
  (set `self.PlayerREF` _asbp_main_player)
  (`KismetSystemLibrary.K2_SetTimerDelegate` (delegate `Test`) 2.0 true))

(event `Test`
  (`/Engine/EditorBlueprintResources/StandardMacros.FlipFlop`
    (:`A`
      (`self.TurnOffLights`))
    (:`B`
      (`self.TurnOnLights`))))

(event `TurnOnLights`
  (`/Game/Blueprints/BP_MainPlayer.UpdateLights` (`self.PlayerREF`) true)
  (`GameplayStatics.PlaySoundAtLocation` "/Game/_Sound/SFX/Lightbreaker_Cue.Lightbreaker_Cue" (`self.K2_GetActorLocation`) (struct) 1.0 1.5 0.0 "/Game/FPSPuzzleSP/Blueprints/Components/SoundAttenuation.SoundAttenuation" null null null))

(event `TurnOffLights`
  (`/Game/Blueprints/BP_MainPlayer.UpdateLights` (`self.PlayerREF`) false)
  (`GameplayStatics.PlaySoundAtLocation` "/Game/_Sound/SFX/Lightbreaker_Cue.Lightbreaker_Cue" (`self.K2_GetActorLocation`) (struct) 1.0 1.0 0.0 "/Game/FPSPuzzleSP/Blueprints/Components/SoundAttenuation.SoundAttenuation" null null null))

(fn `UserConstructionScript`)