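; BP_Level1Crack is a one-shot trigger that collapses a cracked wall when the player enters its box.
; On first overlap it plays a collapse sound, applies a kinematic field to the Wall's geometry collection and spawns a Niagara effect, all centered on its Sphere.
; Timed delays then enable collision on the Floor mesh and later switch off the wall's physics simulation.
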(event `self.Box.OnComponentBeginOverlap`
  (params (OverlappedComponent :type "PrimitiveComponent Object Reference") (OtherActor :type "Actor Object Reference") (OtherComp :type "PrimitiveComponent Object Reference") (OtherBodyIndex :type Integer) (bFromSweep :type Boolean) (SweepResult :type "HitResult Structure (by ref)"))
  (bind _returnvalue_location (`KismetMathLibrary.BreakTransform` (`SceneComponent.K2_GetComponentToWorld` (`self.Sphere`))))
  (bind _geometrycollectioncomponent (`GeometryCollectionActor.GeometryCollectionComponent` (`self.Wall`)))
  (cast `/Game/Blueprints/BP_MainPlayer` OtherActor)
  (`/Engine/EditorBlueprintResources/StandardMacros.DoOnce` false
    (:`Completed`
      (`GameplayStatics.PlaySoundAtLocation` "/Game/_Sound/SFX/WallCollapse.WallCollapse" _returnvalue_location (struct) 1.0 1.0 0.0 "/Game/FPSPuzzleSP/Blueprints/Components/SoundAttenuation.SoundAttenuation" null null null)
      (`GeometryCollectionComponent.ApplyKinematicField` _geometrycollectioncomponent 500.0 _returnvalue_location)
      (`NiagaraFunctionLibrary.SpawnSystemAtLocation` "/Game/_Art/Niagara/NS_Level1Crack.NS_Level1Crack" _returnvalue_location)
      (`KismetSystemLibrary.Delay` 2.5)
      (`PrimitiveComponent.SetCollisionEnabled` (`StaticMeshActor.StaticMeshComponent` (`self.Floor`)) "QueryAndPhysics")
      (`KismetSystemLibrary.Delay` 1.5)
      (`PrimitiveComponent.SetSimulatePhysics` _geometrycollectioncomponent false))))

(fn `UserConstructionScript`)