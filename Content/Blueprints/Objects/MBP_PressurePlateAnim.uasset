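; Animated pressure plate that pulls a Qwob into its socket and signals activation, built on a parent Blueprint.
; ActivateAnim force-ungrabs the Qwob, then chained timelines align it above the final position and lower it as the plate rises, then send activation.
; The Qwob leaving the box stops both timelines, while DeactivateAnim sends deactivation and reverses the plate's motion.
; Signal callbacks switch the ring's dynamic material Strength on and off.
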(event `self.ReceiveBeginPlay`
  (`parent.ReceiveBeginPlay`)
  (bind _returnvalue (`PrimitiveComponent.CreateDynamicMaterialInstance` (`self.PressurePlateRing`) 0 "/Game/Materials/MI_PressurePlateRing.MI_PressurePlateRing" "None"))
  (bind _output_get (set `self.RingMaterial` _returnvalue))
  (`MaterialInstanceDynamic.SetScalarParameterValue` _output_get "Strength" 0.0)
  (set `self.OriginalLocation` (`self.K2_GetActorLocation`)))

(event `self.ActivateAnim`
  (params (QwobMarker :type "PrimitiveComponent Object Reference"))
  (bind (_returnvalue_location _returnvalue_rotation) (`KismetMathLibrary.BreakTransform` (`SceneComponent.K2_GetComponentToWorld` QwobMarker)))
  (bind _originallocation (`self.OriginalLocation`))
  (bind (_returnvalue_location_2 _returnvalue_rotation_2) (`KismetMathLibrary.BreakTransform` (`SceneComponent.K2_GetComponentToWorld` (`self.FinalPosition`))))
  (`/Game/Blueprints/BP_MainPlayer.ForcedUngrab` (`self.PlayerREF`))
  (message `/Game/Blueprints/MBI_ObjectFunctionality.UpdatePhysics` (`self.CurrentQwob`) false)
  (set `self.LocationTemp` _returnvalue_location)
  (set `self.RotationTemp` _returnvalue_rotation)
  (bind (_direction _alpha) (`Timeline|Orient` :!via `PlayFromStart` :!label _label)
    (:`Update`
      (`SceneComponent.K2_SetWorldLocationAndRotation` QwobMarker (`KismetMathLibrary.VLerp` (`self.LocationTemp`) (+ _returnvalue_location_2 (0.0 0.0 100.0)) _alpha) (`KismetMathLibrary.RLerp` (`self.RotationTemp`) _returnvalue_rotation_2 _alpha true) false false))
    (:`Finished`
      (bind _output_get (set `self.LocationTemp` (`SceneComponent.K2_GetComponentLocation` QwobMarker)))
      (bind (_direction_2 _alpha_2) (`Timeline|Timeline` :!via `PlayFromStart` :!label _label_2)
        (:`Update`
          (`SceneComponent.K2_SetWorldLocation` QwobMarker (`KismetMathLibrary.VLerp` _output_get (`SceneComponent.K2_GetComponentLocation` (`self.FinalPosition`)) _alpha_2) false false)
          (`self.K2_SetActorLocation` (`KismetMathLibrary.VLerp` _originallocation (+ _originallocation (0.0 0.0 20.0)) _alpha_2)))
        (:`Finished`
          (`self.SendActivation`))))))

(event `self.Box.OnComponentEndOverlap`
  (params (OverlappedComponent :type "PrimitiveComponent Object Reference") (OtherActor :type "Actor Object Reference") (OtherComp :type "PrimitiveComponent Object Reference") (OtherBodyIndex :type Integer))
  (if (== OtherActor (`self.CurrentQwob`))
    (`|ExecutionSequence`
      (:`then_0`
        (goto _label :!via `Stop`))
      (:`then_1`
        (goto _label_2 :!via `Stop`)))))

(event `self.AfterSignalOn`
  (`MaterialInstanceDynamic.SetScalarParameterValue` (`self.RingMaterial`) "Strength" 2.0))

(event `self.AfterSignalOff`
  (`MaterialInstanceDynamic.SetScalarParameterValue` (`self.RingMaterial`) "Strength" 0.0))

(event `self.DeactivateAnim`
  (bind _originallocation (`self.OriginalLocation`))
  (`self.SendDeactivation`)
  (bind (_direction _alpha) (`Timeline|Timeline_0` :!via `ReverseFromEnd`)
    (:`Update`
      (`self.K2_SetActorLocation` (`KismetMathLibrary.VLerp` _originallocation (+ _originallocation (0.0 0.0 20.0)) _alpha)))))

(fn `UserConstructionScript`
  (`parent.UserConstructionScript`))