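; Big door that, when activated, moves its mesh from its starting location to a Target component's location.
; A Raise timeline, rate-scaled by RiseSeconds, drives the position lerp with teleporting moves while looping-style travel audio plays until it finishes.
; Once playback reaches 1.0, a DoOnce fires the dust Niagara effect and impact sound; timeline completion stops the audio and plays a finish sound.
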(event `self.ReceiveBeginPlay`
  (set `self.OriginalLocation` (`SceneComponent.K2_GetComponentLocation` (`self.Mesh`)))
  (set `self.TargetLocation` (`SceneComponent.K2_GetComponentLocation` (`self.Target`)))
  (`TimelineComponent.SetPlayRate` (`self.Raise`) (/ 1.0 (`self.RiseSeconds`)))
  (`parent.ReceiveBeginPlay`))

(event `self.Activate`
  (bind (_returnvalue_location _returnvalue_rotation) (`KismetMathLibrary.BreakTransform` (`SceneComponent.K2_GetComponentToWorld` (`self.DustSpawn`))))
  (`parent.Activate`)
  (`AudioComponent.Play` (`self.Audio`) 0.0)
  (bind (_direction _alpha) (`Timeline|Raise` :!via `PlayFromStart`)
    (:`Update`
      (`SceneComponent.K2_SetWorldLocation` (`self.Mesh`) (`KismetMathLibrary.VLerp` (`self.OriginalLocation`) (`self.TargetLocation`) _alpha) false true)
      (if (>= (`TimelineComponent.GetPlaybackPosition` (`self.Raise`)) 1.0)
        (`/Engine/EditorBlueprintResources/StandardMacros.DoOnce` false
          (:`Completed`
            (`NiagaraFunctionLibrary.SpawnSystemAtLocation` "/Game/_Art/Niagara/NS_BigDoor.NS_BigDoor" _returnvalue_location _returnvalue_rotation)
            (`GameplayStatics.PlaySoundAtLocation` "/Game/FPSPuzzleSP/Sounds/Wav/S_CubeHit.S_CubeHit" (`SceneComponent.K2_GetComponentLocation` (`self.Mesh`)) (struct) 1.0 1.0 0.0 null null null null)))))
    (:`Finished`
      (`AudioComponent.Stop` (`self.Audio`))
      (`GameplayStatics.PlaySoundAtLocation` (`self.ActiveFinishSFX`) (`SceneComponent.K2_GetComponentLocation` (`self.Mesh`)) (struct) 0.5 1.0 0.0 "/Game/FPSPuzzleSP/Blueprints/Components/SoundAttenuation.SoundAttenuation" null null null))))

(fn `UserConstructionScript`
  (`parent.UserConstructionScript`))