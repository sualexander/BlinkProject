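; BP_StandButton is an interactable button that toggles an active state and relays it to linked actors.
; The construction script puts a dynamic material on the mesh's second slot, and BeginPlay colors it red and tags the mesh.
; Interact flips IsActive, swaps the color between red and grey, and sends the matching TurnMessage to each OutputTo entry.
; The click sound sits inside both loops, playing once per output.
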(event `self.ReceiveBeginPlay`
  (`MaterialInstanceDynamic.SetVectorParameterValue` (`self.Material`) "Color" (struct :`R` 1.0 :`A` 1.0))
  (bind _tags (`/Game/Blueprints/BPL_VisibilityAndTagging.MakeTags` (`|MakeArray` "NewEnumerator5" :!type "/Game/Blueprints/E_Tags Enum")))
  (set `ActorComponent.ComponentTags` _tags (`self.StaticMesh`)))

(event `/Game/Blueprints/BI_Interact.Interact`
  (params (WasGrabbing :type Boolean))
  (if (`self.IsActive`)
    (`MaterialInstanceDynamic.SetVectorParameterValue` (`self.Material`) "Color" (struct :`R` 1.0 :`A` 1.0))
    (set `self.IsActive` false)
    (for _array_element (`self.Output to:`)
      (message `/Game/Blueprints/BI_Signal.Turn` _array_element "NewEnumerator1")
      (`/Game/FPSPuzzleSP/Blueprints/Components/FL_PuzzleLib.PlaySoundByDataTable` "BP_ClickButton" (`self.K2_GetActorLocation`) :!label _label))
    (else
      (set `self.IsActive` true)
      (`MaterialInstanceDynamic.SetVectorParameterValue` (`self.Material`) "Color" (struct :`R` 0.3 :`G` 0.3 :`B` 0.3 :`A` 1.0)) ; Change color then off
      (for _array_element_2 (`self.Output to:`)
        (message `/Game/Blueprints/BI_Signal.Turn` _array_element_2 "NewEnumerator0")
        (goto _label)))))

(fn `UserConstructionScript`
  (bind _returnvalue (`KismetMaterialLibrary.CreateDynamicMaterialInstance` "/Game/FPSPuzzleSP/Materials/Instance/MI_ClickButton.MI_ClickButton"))
  (bind _output_get (set `self.Material` _returnvalue))
  (`PrimitiveComponent.SetMaterial` (`self.StaticMesh`) 1 _output_get))