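; Qwob object that teleports between hidden tagged marker meshes whenever the player is not looking at it or blinks.
; Tick tests visibility using deduplicated, scaled vertices from the first marker's mesh, then searches for an unseen marker, retrying on a looping timer if none is found.
; Candidates are ordered cyclically from the current marker; blinks skip the visibility test.
; Closed eyes pause the Tick check, and Locker locks block both paths.
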(event `self.ReceiveBeginPlay`
  ;[0 0 0] BeginPlay: Initialize Markers and Qwob
  (`|ExecutionSequence`
    (:`then_0`
      (bind _output_get (set `self.Markers` (`self.GetComponentsByTag` "/Script/Engine.StaticMeshComponent" "Marker")))
      (bind _output_get_2 (set `self.NumMarkers` (`KismetArrayLibrary.Array_Length` _output_get)))
      (bind _output_get_3 (set `self.CurrentMarker` (`KismetMathLibrary.RandomInteger` _output_get_2)))
      (`self.GetVertices` _output_get)
      (`self.UpdateQWOB` _output_get_3))
    (:`then_1`
      (for _array_element (`self.Markers`)
        (`SceneComponent.SetHiddenInGame` _array_element true false)))
    (:`then_2`
      (bind _asbp_main_player (cast `/Game/Blueprints/BP_MainPlayer` (`GameplayStatics.GetPlayerPawn` 0)))
      (bind _output_get_4 (set `self.PlayerREF` _asbp_main_player)))))

(event `self.ReceiveTick`
  (params (DeltaSeconds :type "Float (single-precision)"))
  ;[0 0 0] Event Tick: Check whether to update Qwob or not
  (bind _locked (`self.CheckRegularLocks`))
  (if (not _locked)
    (bind _isvisible (`self.IsVisible`))
    (if _isvisible
      (`self.AllowTeleport`)
      (`KismetSystemLibrary.K2_ClearAndInvalidateTimerHandle` (`self.TeleportTimerREF`))
      (else
        (`/Engine/EditorBlueprintResources/StandardMacros.DoOnce` false :!label _label
          (:`Completed`
            (bind (_index _found) (`self.SearchMarkers`))
            (if _found
              (`self.UpdateQWOB` _index)
              (else
                (bind _returnvalue (`KismetSystemLibrary.K2_SetTimerDelegate` (delegate `AllowTeleport`) 0.1 true))
                (set `self.TeleportTimerREF` _returnvalue)))))))))

(event `AllowTeleport`
  ;[0 0 0] Event Tick: Check whether to update Qwob or not
  (goto _label :!via `Reset`))

(event `Blink`
  (bind _indices (`self.Indices`))
  ;[0 0 0] Blink behavior
  (bind _locked (`self.CheckBlinkLocks`))
  (if (not _locked)
    (`self.GenerateIndices` (`self.NumMarkers`))
    (if (> (`KismetArrayLibrary.Array_Length` _indices) 0)
      (`self.UpdateQWOB` (`|GetArrayItem` _indices))
      (else
        (`self.UpdateQWOB` (`KismetArrayLibrary.Array_Random` _indices))))
    (`self.ClosedEyes`)))

(event `Bind to Blink`
  (params (BlinkWidget :type "/Game/Blueprints/BPW_BlinkEffect Object Reference"))
  ;[0 0 0] Blink behavior
  (add `/Game/Blueprints/BPW_BlinkEffect.EyesClosed` BlinkWidget (`|CreateDelegate` :!event `Blink`))
  (add `/Game/Blueprints/BPW_BlinkEffect.EyesOpened` BlinkWidget (delegate `OpenedEyes`)))

(event `OpenedEyes`
  ;[0 0 0] Blink behavior
  (set `self.EyesClosed` false))

(event `ClosedEyes`
  ;[0 0 0] Blink behavior
  (set `self.EyesClosed` true))

(fn `CheckBlinkLocks`
  (returns (Locked :type Boolean))
  ;[0 0 0] Check if locked by Locker
  (if (`self.IsInLocker`)
    (return true)
    (else
      (return false))))

(fn `CheckRegularLocks`
  (returns (Locked :type Boolean))
  ;[0 0 0] Check if eyes are closed, or locked by a Locker
  (if (`self.EyesClosed`)
    (return true)
    (elif (`self.IsInLocker`)
      (return true)
      (else
        (return false)))))

(fn `GenerateIndices`
  (params (NumIndices :type Integer))
  (bind _indices (`self.Indices`))
  (bind _currentmarker (`self.CurrentMarker`))
  ;[0 0 0] Make integer array of element index
  (`KismetArrayLibrary.Array_Clear` _indices)
  (for _index (range NumIndices)
    (`KismetArrayLibrary.Array_Add` _indices (mod (+ _index _currentmarker) NumIndices)))
  (`KismetArrayLibrary.Array_RemoveItem` _indices _currentmarker)
  (return))

(fn `GetVertices`
  (params (Array :type "Array of StaticMeshComponent Object Reference"))
  (bind _output (`|GetArrayItem` Array))
  ;[0 0 0] Stores vertices of mesh, removes duplicates
  (bind _vertices (`KismetProceduralMeshLibrary.GetSectionFromStaticMesh` (`StaticMeshComponent.StaticMesh` _output)))
  (for _array_element _vertices
    (`KismetArrayLibrary.Array_AddUnique` (`self.Vertices`) (* _array_element (`SceneComponent.K2_GetComponentScale` _output)))))

(fn `IsVisible`
  (returns (IsVisible :type Boolean))
  (bind _isvisible (`self.ToObjectRaycast`))
  (if _isvisible
    (return true)
    (else
      (return false))))

(fn `SearchMarkers`
  (returns (Index :type Integer) (Found :type Boolean))
  (locals (CurrIndex :type Integer :default 0))
  (bind _indices (`self.Indices`))
  ;[0 0 0] Search through all markers, return any not visible if any
  (`self.GenerateIndices` (`self.NumMarkers`))
  (while (> (`KismetArrayLibrary.Array_Length` _indices) 0)
    (bind _output_get (set `local.CurrIndex` (`|GetArrayItem` _indices)))
    (bind _output (`|GetArrayItem` _indices _output_get))
    (bind _isvisible (`/Game/Blueprints/AreVerticesVisible.Is Component Visible` (`self.Vertices`) (`|GetArrayItem` (`self.Markers`) _output)))
    (if _isvisible
      (`KismetArrayLibrary.Array_RemoveItem` _indices _output)
      (else
        (return _output true))))
  (return 0 false))

(fn `ToObjectRaycast`
  (returns (IsVisible :type Boolean))
  ;[0 0 0] Calls visibility function on current marker
  (bind _isvisible (`/Game/Blueprints/AreVerticesVisible.Is Component Visible` (`self.Vertices`) (`|GetArrayItem` (`self.Markers`) (`self.CurrentMarker`))))
  (return _isvisible))

(fn `UpdateQWOB`
  (params (Marker :type Integer))
  ;[0 0 0] Teleports Qwob to selected marker
  (bind _output_get (set `self.CurrentMarker` Marker))
  (`SceneComponent.K2_SetWorldLocation` (`self.QWOB`) (`SceneComponent.K2_GetComponentLocation` (`|GetArrayItem` (`self.Markers`) _output_get)) false true)
  (`KismetSystemLibrary.K2_ClearAndInvalidateTimerHandle` (`self.TeleportTimerREF`)))

(fn `UserConstructionScript`)