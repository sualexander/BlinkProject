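; A two-plate puzzle actor that destroys its Target actor, printing "Opened", when both plates are active at the same time.
; Each trigger box activates on overlap by a BP_QwobCyclic and tints its plate's dynamic material with that actor's Color.
; Any end overlap, regardless of actor type, deactivates that plate and resets it to black.
; Every state change calls Update to check both flags.
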(event `self.ReceiveBeginPlay`
  (bind _returnvalue (`PrimitiveComponent.CreateDynamicMaterialInstance` (`self.StaticMesh`) 0 "/Game/Materials/M_PressurePlate.M_PressurePlate" "None"))
  (set `self.Mat0` _returnvalue)
  (bind _returnvalue_2 (`PrimitiveComponent.CreateDynamicMaterialInstance` (`self.StaticMesh1`) 0 "/Game/Materials/M_PressurePlate.M_PressurePlate" "None"))
  (set `self.Mat1` _returnvalue_2))

(event `Update`
  (if (and (`self.IsActive`) (`self.IsActive2`))
    (`KismetSystemLibrary.PrintString` "Opened")
    (`self.K2_DestroyActor` (`self.Target`))))

(event `self.Cube.OnComponentBeginOverlap`
  (params (OverlappedComponent :type "PrimitiveComponent Object Reference") (OtherActor :type "Actor Object Reference") (OtherComp :type "PrimitiveComponent Object Reference") (OtherBodyIndex :type Integer) (bFromSweep :type Boolean) (SweepResult :type "HitResult Structure (by ref)"))
  (bind _asbp_qwob_cyclic (cast `/Game/Blueprints/Objects/BP_QwobCyclic` OtherActor))
  (set `self.IsActive` true)
  (`MaterialInstanceDynamic.SetVectorParameterValue` (`self.Mat0`) "Color" (`/Game/Blueprints/Objects/BP_QwobCyclic.Color` _asbp_qwob_cyclic))
  (`self.Update` :!label _label))

(event `self.Cube.OnComponentEndOverlap`
  (params (OverlappedComponent :type "PrimitiveComponent Object Reference") (OtherActor :type "Actor Object Reference") (OtherComp :type "PrimitiveComponent Object Reference") (OtherBodyIndex :type Integer))
  (set `self.IsActive` false)
  (`MaterialInstanceDynamic.SetVectorParameterValue` :`self` (`self.Mat0`) :`ParameterName` "Color")
  (goto _label))

(event `self.Cube1.OnComponentBeginOverlap`
  (params (OverlappedComponent :type "PrimitiveComponent Object Reference") (OtherActor :type "Actor Object Reference") (OtherComp :type "PrimitiveComponent Object Reference") (OtherBodyIndex :type Integer) (bFromSweep :type Boolean) (SweepResult :type "HitResult Structure (by ref)"))
  (bind _asbp_qwob_cyclic (cast `/Game/Blueprints/Objects/BP_QwobCyclic` OtherActor))
  (set `self.IsActive2` true)
  (`MaterialInstanceDynamic.SetVectorParameterValue` (`self.Mat1`) "Color" (`/Game/Blueprints/Objects/BP_QwobCyclic.Color` _asbp_qwob_cyclic))
  (goto _label))

(event `self.Cube1.OnComponentEndOverlap`
  (params (OverlappedComponent :type "PrimitiveComponent Object Reference") (OtherActor :type "Actor Object Reference") (OtherComp :type "PrimitiveComponent Object Reference") (OtherBodyIndex :type Integer))
  (set `self.IsActive2` false)
  (`MaterialInstanceDynamic.SetVectorParameterValue` :`self` (`self.Mat1`) :`ParameterName` "Color")
  (goto _label))

(fn `UserConstructionScript`)