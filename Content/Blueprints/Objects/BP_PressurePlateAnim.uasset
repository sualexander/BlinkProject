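; Animated pressure plate that pulls a Qwob into place and signals activation, extending a parent class.
; When detection updates while inactive, or activation occurs without the player grabbing, one timeline aligns the Qwob mesh above the target.
; A second timeline lowers it into place while raising the plate, then sends activation; leaving the box stops both.
; Deactivation returns the plate, and signal events toggle the ring's dynamic material glow.
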(event `self.ReceiveBeginPlay`
  (`parent.ReceiveBeginPlay`)
  (bind _returnvalue (`PrimitiveComponent.CreateDynamicMaterialInstance` (`self.PressurePlateRing`) 0 "/Game/Materials/MI_PressurePlateRing.MI_PressurePlateRing" "None"))
  (bind _output_get (set `self.RingMaterial` _returnvalue))
  (`MaterialInstanceDynamic.SetScalarParameterValue` _output_get "Strength" 0.0)
  (set `self.OriginalLocation` (`self.K2_GetActorLocation`))
  (add `/Game/Blueprints/BP_MainPlayer.Ungrabbed` (`self.PlayerREF`) (`|CreateDelegate` :!event `UpdateDetection`)))

(event `UpdateDetection`
  (bind _originallocation (`self.OriginalLocation`))
  (bind _currentqwob (`self.CurrentQwob`))
  (bind (_returnvalue_location _returnvalue_rotation) (`KismetMathLibrary.BreakTransform` (`SceneComponent.K2_GetComponentToWorld` (`self.FinalPosition`))))
  (if (not (`self.IsActive`))
    (`/Engine/EditorBlueprintResources/StandardMacros.IsValid` _currentqwob :!label _label
      (:`Is Valid`
        (message `/Game/Blueprints/BI_ObjectFunctionality.UpdatePhysics` _currentqwob false)
        (bind _tags (`/Game/Blueprints/BPL_VisibilityAndTagging.MakeTags` (`|MakeArray` "NewEnumerator1" :!type "/Game/Blueprints/ENUM_Tags Enum")))
        (bind _output (`|GetArrayItem` (`self.GetComponentsByTag` _currentqwob "/Script/Engine.StaticMeshComponent" (`|GetArrayItem` _tags))))
        (bind (_returnvalue_location_2 _returnvalue_rotation_2) (`KismetMathLibrary.BreakTransform` (`SceneComponent.K2_GetComponentToWorld` _output)))
        (set `self.LocationTemp` _returnvalue_location_2)
        (set `self.RotationTemp` _returnvalue_rotation_2)
        (bind (_direction _alpha) (`Timeline|Orient` :!via `PlayFromStart` :!label _label_2)
          (:`Update`
            (`SceneComponent.K2_SetWorldLocationAndRotation` _output (`KismetMathLibrary.VLerp` (`self.LocationTemp`) (+ _returnvalue_location (0.0 0.0 100.0)) _alpha) (`KismetMathLibrary.RLerp` (`self.RotationTemp`) _returnvalue_rotation _alpha true) false false))
          (:`Finished`
            (bind _output_get (set `self.LocationTemp` (`SceneComponent.K2_GetComponentLocation` _output)))
            (bind (_direction_2 _alpha_2) (`Timeline|Timeline` :!via `PlayFromStart` :!label _label_3)
              (:`Update`
                (`SceneComponent.K2_SetWorldLocation` _output (`KismetMathLibrary.VLerp` _output_get (`SceneComponent.K2_GetComponentLocation` (`self.FinalPosition`)) _alpha_2) false false)
                (`self.K2_SetActorLocation` (`KismetMathLibrary.VLerp` _originallocation (+ _originallocation (0.0 0.0 20.0)) _alpha_2)))
              (:`Finished`
                (`self.SendActivation`)))))))))

(event `self.ActivateAnim`
  (if (not (`/Game/Blueprints/BP_MainPlayer.IsGrabbing` (`self.PlayerREF`)))
    (goto _label)))

(event `self.Box.OnComponentEndOverlap`
  (params (OverlappedComponent :type "PrimitiveComponent Object Reference") (OtherActor :type "Actor Object Reference") (OtherComp :type "PrimitiveComponent Object Reference") (OtherBodyIndex :type Integer))
  (if (== OtherActor (`self.CurrentQwob`))
    (`|ExecutionSequence`
      (:`then_0`
        (goto _label_2 :!via `Stop`))
      (:`then_1`
        (goto _label_3 :!via `Stop`)))))

(event `self.AfterSignalOn`
  (`MaterialInstanceDynamic.SetScalarParameterValue` (`self.RingMaterial`) "Strength" 2.0))

(event `self.AfterSignalOff`
  (`MaterialInstanceDynamic.SetScalarParameterValue` (`self.RingMaterial`) "Strength" 0.0))

(event `self.DeactivateAnim`
  (bind _originallocation (`self.OriginalLocation`))
  (`self.SendDeactivation`)
  (bind (_direction _alpha) (`Timeline|Timeline_0` :!via `ReverseFromEnd`)
    (:`Update`
      (`self.K2_SetActorLocation` (`KismetMathLibrary.VLerp` _originallocation (+ _originallocation (0.0 0.0 20.0)) _alpha)))))

(fn `UserConstructionScript`
  (`parent.UserConstructionScript`))