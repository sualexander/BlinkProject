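; LevelTransitioner is an actor that swaps streamed levels once, triggered by a visibility check on its static mesh.
; Tick passes its first static mesh component to IsTransitionVisible until that returns true, then sets Switched so the swap does not repeat.
; It loads LevelTo and unloads LevelFrom, with SafeLoad controlling blocking, then calls CallFinishedInit on BP_MainPlayer.
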(event `self.ReceiveTick`
  (params (DeltaSeconds :type "Float (single-precision)"))
  (if (not (`self.Switched`))
    (bind _isvisible (`/Game/Blueprints/BPL_VisibilityAndTagging.Is Transition Visible` (`|MakeArray` (0.0 0.0 0.0) :!type "Vector Structure") (`|GetArrayItem` (`self.K2_GetComponentsByClass` "/Script/Engine.StaticMeshComponent"))))
    (if _isvisible
      (set `self.Switched` true)
      (`GameplayStatics.LoadStreamLevel` (`KismetStringLibrary.Conv_StringToName` (`self.LevelTo`)) true (`self.SafeLoad`))
      (`GameplayStatics.UnloadStreamLevel` (`KismetStringLibrary.Conv_StringToName` (`self.LevelFrom`)) (`self.SafeLoad`))
      (bind _asbp_main_player (cast `/Game/Blueprints/BP_MainPlayer` (`GameplayStatics.GetPlayerCharacter` 0)))
      (`/Game/Blueprints/BP_MainPlayer.FinishedInit` _asbp_main_player))))

(fn `UserConstructionScript`)