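; LightBreaker is an object Blueprint that switches lights on or off by way of the player.
; At BeginPlay it caches the BP_MainPlayer reference, and its TurnOnLights and TurnOffLights events pass true or false to that player's UpdateLights.
; Delay chains for timed on and off switching are present but disconnected, so the events fire only when called.
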(event `self.ReceiveBeginPlay`
  (bind _asbp_main_player (cast `/Game/Blueprints/BP_MainPlayer` (`GameplayStatics.GetPlayerCharacter` 0)))
  (set `self.PlayerREF` _asbp_main_player))

(event `TurnOnLights`
  (`/Game/Blueprints/BP_MainPlayer.UpdateLights` (`self.PlayerREF`) true))

(event `TurnOffLights`
  (`/Game/Blueprints/BP_MainPlayer.UpdateLights` (`self.PlayerREF`) false))

(fn `UserConstructionScript`)