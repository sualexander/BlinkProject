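; Laser emitter that powers a BP_Door it points at, but only while its QWOB mesh is fully visible to the player.
; Each tick, cached mesh vertices, offset by location only, are screen-projected and line-traced from the camera to confirm full visibility.
; Visibility turns the material green and starts a looping forward trace that activates a hit door.
; Losing visibility greys it, stops the timer and deactivates the door, as does losing the door.
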(event `self.ReceiveBeginPlay`
  (bind _qwob (`self.QWOB`))
  (`|ExecutionSequence`
    (:`then_0`
      (bind _vertices (`KismetProceduralMeshLibrary.GetSectionFromStaticMesh` (`StaticMeshComponent.StaticMesh` _qwob)))
      (for _array_element _vertices
        (`KismetArrayLibrary.Array_AddUnique` (`self.Vertices`) _array_element)))
    (:`then_1`
      (bind _returnvalue (`PrimitiveComponent.CreateDynamicMaterialInstance` _qwob 0 "/Game/Materials/MI_SingularLaser.MI_SingularLaser" "None"))
      (set `self.Material` _returnvalue))))

(event `self.ReceiveTick`
  (params (DeltaSeconds :type "Float (single-precision)"))
  (bind _material (`self.Material`))
  (bind _isvisible (`self.IsFullyVisible`))
  (if (xor _isvisible (`self.IsVisible`))
    (bind _output_get (set `self.IsVisible` _isvisible))
    (if _output_get
      (`MaterialInstanceDynamic.SetVectorParameterValue` _material "Color" (struct :`R` 0.384314 :`G` 1.0 :`B` 0.32549 :`A` 1.0))
      (bind _returnvalue (`KismetSystemLibrary.K2_SetTimerDelegate` (delegate `CheckLOS`) 0.1 true))
      (set `self.LOSTimer` _returnvalue)
      (else
        (`MaterialInstanceDynamic.SetVectorParameterValue` _material "Color" (struct :`R` 0.208333 :`G` 0.208333 :`B` 0.208333 :`A` 1.0))
        (`KismetSystemLibrary.K2_ClearAndInvalidateTimerHandle` (`self.LOSTimer`))
        (set `self.Has LOS` false)
        (bind _asbp_door (cast `/Game/Blueprints/Objects/BP_Door` (`self.HitPortal`) :!label _label))
        (`/Game/Blueprints/Objects/BP_Door.Deactivate` _asbp_door)))))

(event `CheckLOS`
  (bind _haslos (`self.CanSeePortal`))
  (if (xor _haslos (`self.Has LOS`))
    (bind _output_get (set `self.Has LOS` _haslos))
    (if _output_get
      (bind _asbp_door (cast `/Game/Blueprints/Objects/BP_Door` (`self.HitPortal`)))
      (`/Game/Blueprints/Objects/BP_Door.Activate` _asbp_door)
      (else
        (goto _label)))))

(fn `CanSeePortal`
  (returns (HasLOS :type Boolean))
  (bind _returnvalue (`SceneComponent.K2_GetComponentLocation` (`self.Sphere`)))
  (bind (_outhit _returnvalue_2) (`KismetSystemLibrary.LineTraceSingleForObjects` :`Start` _returnvalue :`End` (+ _returnvalue (* (`self.GetActorForwardVector`) 5000)) :`ObjectTypes` (`|MakeArray` "ObjectTypeQuery1" "ObjectTypeQuery2" :!type "EObjectTypeQuery Enum") :`DrawDebugType` "ForDuration" :`TraceColor` (struct :`R` 1.0 :`G` 0.052705 :`A` 1.0) :`DrawTime` 0.1))
  (if _returnvalue_2
    (bind (_bblockinghit _binitialoverlap _time _distance _location _impactpoint _normal _impactnormal _physmat _hitactor) (`GameplayStatics.BreakHitResult` _outhit))
    (if (== (`GameplayStatics.GetObjectClass` _hitactor) "/Game/Blueprints/Objects/BP_Door.BP_Door_C")
      (set `self.HitPortal` _hitactor)
      (return true)
      (else
        _)))
  (return false))

(fn `IsFullyInFOV`
  (returns (InFOV :type Boolean))
  (locals (IsInFOV :type Boolean))
  (for _array_element (`self.Vertices`)
    (bind _infov (`self.IsPointFullyInFOV` (+ _array_element (`SceneComponent.K2_GetComponentLocation` (`self.QWOB`)))))
    (if (not _infov)
      (return false)))
  (return true))

(fn `IsFullyVisible`
  (returns (IsVisible :type Boolean))
  (locals (Theta :type "Float (double-precision)"))
  (bind _returnvalue (`SceneComponent.K2_GetComponentLocation` (`self.QWOB`)))
  (bind _infov (`self.IsFullyInFOV`))
  (if _infov
    (for _array_element (`self.Vertices`)
      (bind _returnvalue_2 (+ _array_element _returnvalue))
      (bind (_outhit _returnvalue_3) (`KismetSystemLibrary.LineTraceSingleForObjects` :`Start` (`self.K2_GetActorLocation` (`GameplayStatics.GetPlayerCameraManager` 0)) :`End` (+ _returnvalue_2 (* (`KismetMathLibrary.Normal` (- _returnvalue _returnvalue_2)) 2)) :`ObjectTypes` (`|MakeArray` "ObjectTypeQuery2" "ObjectTypeQuery1" :!type "EObjectTypeQuery Enum") :`bIgnoreSelf` false :`DrawTime` 0.5))
      (if (not (and _returnvalue_3 (== (`.HitComponent` (`GameplayStatics.BreakHitResult` _outhit)) (`self.QWOB`))))
        (return false)))
    (return true)
    (else
      (return false))))

(fn `IsPointFullyInFOV`
  (params (Point :type "Vector Structure"))
  (returns (InFOV :type Boolean))
  (bind (_returnvalue_x _returnvalue_y) (`KismetMathLibrary.BreakVector2D` (`WidgetLayoutLibrary.GetViewportSize`)))
  (bind _screenlocation (`PlayerController.ProjectWorldLocationToScreen` (`GameplayStatics.GetPlayerController` 0) Point false))
  (return (and (> (`KismetMathLibrary.BreakVector2D` _screenlocation) 0.0) (> (`.Y` (`KismetMathLibrary.BreakVector2D` _screenlocation)) 0.0) (< (`KismetMathLibrary.BreakVector2D` _screenlocation) _returnvalue_x) (< (`.Y` (`KismetMathLibrary.BreakVector2D` _screenlocation)) _returnvalue_y))))

(fn `UserConstructionScript`)