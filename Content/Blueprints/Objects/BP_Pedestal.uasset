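; BP_Pedestal is a pedestal that detects whether a tagged Qwob component rests in its box and shows its Quob mesh only while empty.
; A delayed initial overlap check and box overlap events set the presence state, ignoring the player's grabbed actor on entry, and Tick updates mesh visibility.
; BeginPlay applies colored emissive dynamic materials to two cylinders and caches the player, retrying by timer if the cast fails.
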(event `self.ReceiveBeginPlay`
  (bind _color (`self.Color`))
  (bind _asbp_main_player (cast `/Game/Blueprints/BP_MainPlayer` (`GameplayStatics.GetPlayerCharacter` 0))
    (:`then`
      (set `self.PlayerREF` _asbp_main_player)
      (`|ExecutionSequence`
        (:`then_0`
          (`KismetSystemLibrary.Delay` 0.2)
          (bind (_hasinitialoverlap _array_element) (`self.CHeckInitialOverlap`))
          (if _hasinitialoverlap
            (set `self.Qwob` _array_element)
            (set `self.QwobPresent` true :!label _label)))
        (:`then_1`
          (bind _returnvalue (`PrimitiveComponent.CreateDynamicMaterialInstance` (`self.Cylinder1`) 0 "/Game/Materials/MI_EmissiveDoor.MI_EmissiveDoor" "None"))
          (`MaterialInstanceDynamic.SetVectorParameterValue` _returnvalue "Color" _color)
          (bind _returnvalue_2 (`PrimitiveComponent.CreateDynamicMaterialInstance` (`self.Cylinder`) 0 "/Game/Materials/MI_EmissiveDoor.MI_EmissiveDoor" "None"))
          (`MaterialInstanceDynamic.SetVectorParameterValue` _returnvalue_2 "Color" _color))
        (:`then_2`
          (`KismetSystemLibrary.K2_SetTimerDelegate` (`|CreateDelegate` :!event `Switcheroo`) 1.0 true))))
    (:`CastFailed`
      (bind _returnvalue_3 (`KismetSystemLibrary.K2_SetTimerDelegate` (delegate `GetPlayer`) 0.5 true))
      (bind _output_get (set `self.TimerREF` _returnvalue_3)))))

(event `GetPlayer`
  (bind _asbp_main_player (cast `/Game/Blueprints/BP_MainPlayer` (`GameplayStatics.GetPlayerCharacter` 0)))
  (set `self.PlayerREF` _asbp_main_player)
  (`KismetSystemLibrary.K2_ClearAndInvalidateTimerHandle` (stale `self.ReceiveBeginPlay` _output_get)))

(event `Switcheroo`
  (`/Engine/EditorBlueprintResources/StandardMacros.FlipFlop`
    (:`A`
      (set `self.Offset` 1.0))
    (:`B`
      (set `self.Offset` -1.0))))

(event `self.Box.OnComponentBeginOverlap`
  (params (OverlappedComponent :type "PrimitiveComponent Object Reference") (OtherActor :type "Actor Object Reference") (OtherComp :type "PrimitiveComponent Object Reference") (OtherBodyIndex :type Integer) (bFromSweep :type Boolean) (SweepResult :type "HitResult Structure (by ref)"))
  (bind _hastag (`/Game/Blueprints/BPL_VisibilityAndTagging.CheckTag` "NewEnumerator1" (`ActorComponent.ComponentTags` OtherComp)))
  (if (and _hastag (!= (`/Game/Blueprints/BP_MainPlayer.GrabbedActor` (`self.PlayerREF`)) OtherActor))
    (set `self.Qwob` OtherComp)
    (set `self.Other Actor` OtherActor)
    (goto _label)))

(event `self.Box.OnComponentEndOverlap`
  (params (OverlappedComponent :type "PrimitiveComponent Object Reference") (OtherActor :type "Actor Object Reference") (OtherComp :type "PrimitiveComponent Object Reference") (OtherBodyIndex :type Integer))
  (if (== OtherComp (`self.Qwob`))
    (set `self.QwobPresent` false)
    (set `self.Qwob` null)
    (`KismetSystemLibrary.PrintString` "Hello")))

(event `self.ReceiveTick`
  (params (DeltaSeconds :type "Float (single-precision)"))
  (bind _quobfinalhighpoly (`self.QuobFINALHighPoly`))
  (if (`self.QwobPresent`)
    (`SceneComponent.SetVisibility` _quobfinalhighpoly false false)
    (else
      (`SceneComponent.SetVisibility` _quobfinalhighpoly true false))))

(fn `CHeckInitialOverlap`
  (returns (HasInitialOverlap :type Boolean) (`Array Element` :type "PrimitiveComponent Object Reference"))
  (for _array_element (`PrimitiveComponent.GetOverlappingComponents` (`self.Box`))
    (bind _hastag (`/Game/Blueprints/BPL_VisibilityAndTagging.CheckTag` "NewEnumerator1" (`ActorComponent.ComponentTags` _array_element)))
    (if _hastag
      (return true _array_element)))
  (return false null))

(fn `UserConstructionScript`)