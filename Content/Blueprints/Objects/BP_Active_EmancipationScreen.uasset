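; Switchable emancipation screen that releases the player's held object and sends an emancipate message to tagged actors that touch it.
; While active, a Wall overlap checks the actor's static mesh components for the tag, then calls ForcedUngrab on the player and EmancipateMessage on the actor.
; Update counts On/Off signals against a positive threshold; reaching it flips the screen from its StartOn state, and dropping below restores it.
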(event `self.ReceiveBeginPlay`
  (set `self.isActive` (`self.StartOn`))
  (bind _tags (`/Game/Blueprints/BPL_VisibilityAndTagging.MakeTags` (`|MakeArray` "NewEnumerator1" :!type "/Game/Blueprints/ENUM_Tags Enum")))
  (set `self.TagToCheck` (`|GetArrayItem` _tags))
  (bind _asbp_main_player (cast `/Game/Blueprints/BP_MainPlayer` (`GameplayStatics.GetPlayerCharacter` 0)))
  (set `self.PlayerREF` _asbp_main_player))

(event `self.Wall.OnComponentBeginOverlap`
  (params (OverlappedComponent :type "PrimitiveComponent Object Reference") (OtherActor :type "Actor Object Reference") (OtherComp :type "PrimitiveComponent Object Reference") (OtherBodyIndex :type Integer) (bFromSweep :type Boolean) (SweepResult :type "HitResult Structure (by ref)"))
  (if (`self.isActive`)
    (if (> (`KismetArrayLibrary.Array_Length` (`self.GetComponentsByTag` OtherActor "/Script/Engine.StaticMeshComponent" (`self.TagToCheck`))) 0)
      (`/Game/Blueprints/BP_MainPlayer.ForcedUngrab` (`self.PlayerREF`))
      (message `/Game/Blueprints/MBI_ObjectFunctionality.Emancipate` OtherActor))))

(event `Turn On`
  (if (not (`self.isActive`))
    (`KismetSystemLibrary.PrintString` "TURN ON")
    (set `self.isActive` true)))

(event `Turn Off`
  (if (`self.isActive`)
    (`KismetSystemLibrary.PrintString` "Turn oFF")
    (set `self.isActive` false)))

(event `/Game/Blueprints/BI_Signal.Update`
  (params (Signal :type "/Game/FPSPuzzleSP/Blueprints/Components/Enum_Signal Enum" :default "NewEnumerator0"))
  (bind _starton (`self.StartOn`))
  (bind _totalsignals (`self.TotalSignals`))
  (if (<= (`self.SignalThreshold`) 0)
    (switch `/Game/FPSPuzzleSP/Blueprints/Components/Enum_Signal` Signal)
    (else
      (switch `/Game/FPSPuzzleSP/Blueprints/Components/Enum_Signal` Signal
        (:`NewEnumerator0`
          (`/Engine/EditorBlueprintResources/StandardMacros.IncrementInt` _totalsignals
            (:`  `
              _)))
        (:`NewEnumerator1`
          (`/Engine/EditorBlueprintResources/StandardMacros.DecrementInt` _totalsignals
            (:`  `
              _))))
      (if (>= _totalsignals (`self.SignalThreshold`))
        (if _starton
          (`self.Turn Off`)
          (else
            (`self.Turn On`)))
        (elif _starton
          (`self.Turn On`)
          (else
            (`self.Turn Off`)))))))

(fn `UserConstructionScript`)