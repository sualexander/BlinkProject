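; BP_ObjectSingular is a toggleable object that appears or disappears in response to On/Off signals.
; Turn keeps a signal count, clamped at zero on Off, prints it, and compares it with SignalThreshold, with Invert flipping the result.
; Activate and Deactivate set the Mesh's visibility and collision together.
; BeginPlay picks the starting state from IsInitiallyOn, independent of the count.
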(event `self.ReceiveBeginPlay`
  (if (`self.IsInitiallyOn`)
    (`self.Activate`)
    (else
      (`self.Deactivate`))))

(event `Activate`
  (bind _mesh (`self.Mesh`))
  (`PrimitiveComponent.SetCollisionEnabled` _mesh "QueryAndPhysics")
  (`SceneComponent.SetHiddenInGame` _mesh false false))

(event `Deactivate`
  (bind _mesh (`self.Mesh`))
  (`PrimitiveComponent.SetCollisionEnabled` _mesh "NoCollision")
  (`SceneComponent.SetHiddenInGame` _mesh true false))

(event `/Game/Blueprints/BI_Signal.Turn`
  (params (Signal :type "/Game/FPSPuzzleSP/Blueprints/Components/Enum_Signal Enum" :default "NewEnumerator0"))
  (bind _totalsignals (`self.TotalSignals`))
  (bind _invert (`self.Invert`))
  (bind _totalsignals_2 (`self.totalSignals`))
  (switch `/Game/FPSPuzzleSP/Blueprints/Components/Enum_Signal` Signal
    (:`NewEnumerator0`
      (`/Engine/EditorBlueprintResources/StandardMacros.IncrementInt` _totalsignals
        (:`  `
          _)))
    (:`NewEnumerator1`
      (bind _result (`/Engine/EditorBlueprintResources/StandardMacros.DecrementInt` _totalsignals)
        (:`  `
          (if (< _result 0)
            (set `self.TotalSignals` 0))))))
  (`KismetSystemLibrary.PrintString` (`KismetStringLibrary.Conv_IntToString` _totalsignals_2))
  (if (>= _totalsignals_2 (`self.SignalThreshold`))
    (if _invert
      (`self.Deactivate`)
      (else
        (`self.Activate`)))
    (elif _invert
      (`self.Activate`)
      (else
        (`self.Deactivate`)))))

(fn `UserConstructionScript`)