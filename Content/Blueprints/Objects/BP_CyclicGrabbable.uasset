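; Grabbable object that relocates among tagged, hidden marker meshes when out of the player's view, starting at a random one.
; While its Tick gate is open, it tests visibility using cached mesh vertices and jumps once to a random unseen marker, re-arming when seen again.
; With no free marker it starts a retry timer.
; Grab events toggle camera attachment and the gate; Blink forces a random jump and pauses checks until EndBlink.
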(event `self.ReceiveBeginPlay`
  (bind _markers (`self.Markers`))
  (`|ExecutionSequence`
    (:`then_0`
      (bind _output_get (set `self.Markers` (`self.GetComponentsByTag` "/Script/Engine.StaticMeshComponent" "Marker")))
      (bind _output_get_2 (set `self.NumMarkers` (`KismetArrayLibrary.Array_Length` _markers)))
      (bind _output_get_3 (set `self.CurrentMarker` (`KismetMathLibrary.RandomInteger` _output_get_2)))
      (`self.TeleportQWOB` (`|GetArrayItem` _markers _output_get_3)))
    (:`then_1`
      (bind _vertices (`KismetProceduralMeshLibrary.GetSectionFromStaticMesh` (`StaticMeshComponent.StaticMesh` (`|GetArrayItem` _markers))))
      (for _array_element _vertices
        (`KismetArrayLibrary.Array_AddUnique` (`self.Vertices`) _array_element)))
    (:`then_2`
      (add `/Game/Blueprints/GrabComponent.AttachComponents` (`self.GrabComponent`) (delegate `OnGrabbed`))
      (bind _asbp_main_player (cast `/Game/Blueprints/BP_MainPlayer` (`GameplayStatics.GetPlayerPawn` 0)))
      (set `self.PlayerREF` _asbp_main_player)
      (`NiagaraComponent.SetVariableLinearColor` (`self.InsideSphere`) "Color" (`self.Color`)))
    (:`then_3`
      (for _array_element_2 _output_get
        (`SceneComponent.SetHiddenInGame` _array_element_2 true false)))))

(event `OnGrabbed`
  (if (`/Game/Blueprints/GrabComponent.Is Grabbing` (`self.GrabComponent`))
    (`SceneComponent.K2_DetachFromComponent` (`self.QWOB`) "KeepWorld" "KeepWorld" "KeepWorld" true)
    (goto _label :!via `Open`)
    (else
      (`SceneComponent.K2_AttachToComponent` (`self.QWOB`) (`/Game/Blueprints/BP_MainPlayer.Camera` (`self.PlayerREF`)) "None" "KeepWorld" "KeepWorld" "KeepWorld" true)
      (set `self.CurrentMarker` -1)
      (goto _label :!via `Close`))))

(event `self.ReceiveTick`
  (params (DeltaSeconds :type "Float (single-precision)"))
  (`/Engine/EditorBlueprintResources/StandardMacros.Gate` false :!label _label
    (:`Exit`
      (bind _isvisible (`/Game/Blueprints/AreVerticesVisible.Is Component Visible` (`self.Vertices`) (`self.QWOB`)))
      (if _isvisible
        (`self.AllowTeleport`)
        (else
          (`/Engine/EditorBlueprintResources/StandardMacros.DoOnce` false :!label _label_2
            (:`Completed`
              (bind (_index _found) (`self.SearchMarkers`))
              (if _found
                (bind _output_get (set `self.CurrentMarker` _index))
                (`self.TeleportQWOB` (`|GetArrayItem` (`self.Markers`) _output_get))
                (`KismetSystemLibrary.K2_ClearAndInvalidateTimerHandle` (`self.TeleportTimerREF`))
                (else
                  (bind _returnvalue (`KismetSystemLibrary.K2_SetTimerDelegate` (`|CreateDelegate` :!event `AllowTeleport`) 0.1 true))
                  (set `self.TeleportTimerREF` _returnvalue))))))))))

(event `AllowTeleport`
  (goto _label_2 :!via `Reset`))

(event `EndBlink`
  (goto _label :!via `Open`))

(event `Blink`
  (`|ExecutionSequence`
    (:`then_0`
      (bind _marker (`self.RandomMarker`))
      (`self.TeleportQWOB` _marker))
    (:`then_1`
      (goto _label :!via `Close`))))

(event `TeleportQWOB`
  (params (QWOB :type "StaticMeshComponent Object Reference"))
  (`SceneComponent.K2_SetWorldLocation` (`self.QWOB`) (`SceneComponent.K2_GetComponentLocation` QWOB) false false))

(fn `GenerateIndices`
  (params (NumIndices :type Integer))
  (bind _indices (`self.Indices`))
  (`KismetArrayLibrary.Array_Clear` _indices)
  (for _index (range NumIndices)
    (`KismetArrayLibrary.Array_Add` _indices _index))
  (`KismetArrayLibrary.Array_RemoveItem` _indices (`self.CurrentMarker`))
  (return))

(fn `RandomMarker`
  (returns (Marker :type "StaticMeshComponent Object Reference"))
  (locals (RandomIndex :type Integer))
  (bind _nummarkers (`self.NumMarkers`))
  (`self.GenerateIndices` _nummarkers)
  (while (> (`KismetArrayLibrary.Array_Length` (`self.Indices`)) 0)
    (bind _output_get (set `local.RandomIndex` (`KismetMathLibrary.RandomInteger` _nummarkers)))
    (bind _output (`|GetArrayItem` (`self.Indices`) _output_get))
    (if (not (== (`self.CurrentMarker`) _output))
      (bind _output_get_2 (set `self.CurrentMarker` _output))
      (return (`|GetArrayItem` (`self.Markers`) _output_get_2))))
  (`KismetSystemLibrary.PrintString` "YOU DUN FUCKED UP BIG TIME")
  (return null))

(fn `SearchMarkers`
  (returns (Index :type Integer) (Found :type Boolean))
  (locals (RandomIndex :type Integer :default 0))
  (bind _indices (`self.Indices`))
  (bind _returnvalue (`KismetArrayLibrary.Array_Length` _indices))
  (`self.GenerateIndices` (`self.NumMarkers`))
  (while (> _returnvalue 0)
    (bind _output_get (set `local.RandomIndex` (`KismetMathLibrary.RandomInteger` _returnvalue)))
    (bind _output (`|GetArrayItem` _indices _output_get))
    (bind _isvisible (`/Game/Blueprints/AreVerticesVisible.Is Component Visible` (`self.Vertices`) (`|GetArrayItem` (`self.Markers`) _output)))
    (if _isvisible
      (`KismetArrayLibrary.Array_RemoveItem` _indices _output)
      (else
        (return _output true))))
  (return 0 false))

(fn `UserConstructionScript`)