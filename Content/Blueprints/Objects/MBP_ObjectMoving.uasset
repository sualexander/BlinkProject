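; Activatable object Blueprint that moves its mesh between its starting location and a Target's location, both cached at BeginPlay.
; Activate plays the MoveObject timeline, rate-scaled by Seconds, to lerp the mesh with unswept teleports; Deactivate reverses it.
; Looping or travel audio plays during movement, then a state-specific finish sound plays at the mesh.
; Deactivate clears IsActive immediately but defers the parent's deactivation until the timeline finishes.
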(event `self.ReceiveBeginPlay`
  (set `self.OriginalLocation` (`SceneComponent.K2_GetComponentLocation` (`self.Mesh`)))
  (set `self.TargetLocation` (`SceneComponent.K2_GetComponentLocation` (`self.Target`)))
  (`TimelineComponent.SetPlayRate` (`self.MoveObject`) (/ 1.0 (`self.Seconds`)))
  (`parent.ReceiveBeginPlay`))

(event `self.Activate`
  (bind _audio (`self.Audio`))
  (bind _returnvalue (`SceneComponent.K2_GetComponentLocation` (`self.Mesh`)))
  (`parent.Activate`)
  (`AudioComponent.Play` (`self.Audio`) 0.0)
  (bind (_direction _alpha) (`Timeline|MoveObject` :!label _label)
    (:`Update`
      (`SceneComponent.K2_SetWorldLocation` (`self.Mesh`) (`KismetMathLibrary.VLerp` (`self.OriginalLocation`) (`self.TargetLocation`) _alpha) false true))
    (:`Finished`
      (if (`self.IsActive`)
        (`AudioComponent.Stop` _audio)
        (`GameplayStatics.PlaySoundAtLocation` (`self.ActiveFinishSFX`) _returnvalue (struct) 0.5 1.0 0.0 "/Game/FPSPuzzleSP/Blueprints/Components/SoundAttenuation.SoundAttenuation" null null null)
        (else
          (`parent.Deactivate`)
          (`AudioComponent.Stop` _audio)
          (`GameplayStatics.PlaySoundAtLocation` (`self.DeactivateFinishSFX `) _returnvalue (struct) 0.5 0.5 0.0 "/Game/FPSPuzzleSP/Blueprints/Components/SoundAttenuation.SoundAttenuation" null null null))))))

(event `self.Deactivate`
  (set `self.IsActive` false)
  (`AudioComponent.Play` (`self.Audio`) 0.0)
  (goto _label :!via `Reverse`))

(fn `UserConstructionScript`
  (`parent.UserConstructionScript`))