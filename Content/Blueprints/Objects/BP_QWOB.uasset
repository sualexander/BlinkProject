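; BP_QWOB is an object that jumps between mesh components tagged "Marker" when the player is not observing it.
; It picks a random marker at start, and Tick, gated off between Blink and EndBlink, moves it to an unseen marker once the current one leaves view.
; Blink moves it to a random other marker regardless of visibility.
; Visibility combines screen projection of six bounds points with a camera-facing ring of line traces to detect occlusion.
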(event `self.ReceiveBeginPlay`
  (bind _markers (`self.Markers`))
  (`|ExecutionSequence`
    (:`then_0`
      (set `self.Markers` (`self.GetComponentsByTag` "/Script/Engine.StaticMeshComponent" "Marker"))
      (bind _output_get (set `self.NumMarkers` (`KismetArrayLibrary.Array_Length` _markers)))
      (bind _output_get_2 (set `self.CurrentMarker` (`KismetMathLibrary.RandomInteger` _output_get)))
      (`self.TeleportQWOB` (`|GetArrayItem` _markers _output_get_2)))))

(event `self.ReceiveTick`
  (params (DeltaSeconds :type "Float (single-precision)"))
  (`/Engine/EditorBlueprintResources/StandardMacros.Gate` false :!label _label
    (:`Exit`
      (bind _isvisible (`self.ComponentIsVisible` (`|GetArrayItem` (`self.Markers`) (`self.CurrentMarker`)) 30.0))
      (if _isvisible
        (`self.AllowTeleport`)
        (else
          (`/Engine/EditorBlueprintResources/StandardMacros.DoOnce` false :!label _label_2
            (:`Completed`
              (bind (_index _found) (`self.SearchMarkers`))
              (if _found
                (bind _output_get (set `self.CurrentMarker` _index))
                (`self.TeleportQWOB` (`|GetArrayItem` (`self.Markers`) _output_get))
                (else
                  (`KismetSystemLibrary.PrintString` "No Available Spots!"))))))))))

(event `AllowTeleport`
  (goto _label_2 :!via `Reset`))

(event `EndBlink`
  (goto _label :!via `Open`))

(event `Blink`
  (`|ExecutionSequence`
    (:`then_0`
      (bind _marker (`self.RandomMarker`))
      (`self.TeleportQWOB` _marker))
    (:`then_1`
      (goto _label :!via `Close`))))

(event `TeleportQWOB`
  (params (QWOB :type "StaticMeshComponent Object Reference"))
  (`SceneComponent.K2_SetWorldLocation` (`self.QWOB`) (`SceneComponent.K2_GetComponentLocation` QWOB) false false)
  (`KismetSystemLibrary.PrintString` "teleported"))

(fn `ComponentInFOV`
  (params (Component :type "StaticMeshComponent Object Reference"))
  (returns (InFOV :type Boolean))
  (bind (_origin _boxextent _sphereradius) (`KismetSystemLibrary.GetComponentBounds` Component))
  (bind _returnvalue (`SceneComponent.GetUpVector` Component))
  (bind _returnvalue_2 (`SceneComponent.GetRightVector` Component))
  (bind _returnvalue_3 (`SceneComponent.GetForwardVector` Component))
  (bind _hit (`self.PointIsOnScreen` (+ _origin (* _returnvalue _sphereradius)))
    (:`exec`
      (bind _hit_2 (`self.PointIsOnScreen` (+ _origin (* (`KismetMathLibrary.NegateVector` _returnvalue) _sphereradius)))
        (:`exec`
          (bind _hit_3 (`self.PointIsOnScreen` (+ _origin (* _returnvalue_2 _sphereradius)))
            (:`exec`
              (bind _hit_4 (`self.PointIsOnScreen` (+ _origin (* (`KismetMathLibrary.NegateVector` _returnvalue_2) _sphereradius)))
                (:`exec`
                  (bind _hit_5 (`self.PointIsOnScreen` (+ _origin (* _returnvalue_3 _sphereradius)))
                    (:`exec`
                      (bind _hit_6 (`self.PointIsOnScreen` (+ _origin (* (`KismetMathLibrary.NegateVector` _returnvalue_3) _sphereradius)))
                        (:`exec`
                          (return (or _hit _hit_2 _hit_3 _hit_4 _hit_5 _hit_6)))))))))))))))

(fn `ComponentIsVisible`
  (params (Component :type "StaticMeshComponent Object Reference") (Resolution :type "Float (double-precision)"))
  (returns (IsVisible :type Boolean))
  (locals (Theta :type "Float (double-precision)"))
  (bind _returnvalue (`GameplayStatics.GetPlayerCameraManager` 0))
  (bind (_origin _boxextent _sphereradius) (`KismetSystemLibrary.GetComponentBounds` Component))
  (bind _theta (`local.Theta`))
  (bind _infov (`self.ComponentInFOV` Component))
  (if _infov
    (while (<= _theta 360.0)
      (bind (_outhit _returnvalue_2) (`KismetSystemLibrary.LineTraceSingleForObjects` :`Start` (`self.K2_GetActorLocation` _returnvalue) :`End` (+ _origin (`KismetMathLibrary.RotateAngleAxis` (* (`self.GetActorUpVector` _returnvalue) _sphereradius 0.95) _theta (`self.GetActorForwardVector` _returnvalue))) :`ObjectTypes` (`|MakeArray` "ObjectTypeQuery2" :!type "EObjectTypeQuery Enum") :`bIgnoreSelf` false :`DrawTime` 0.5))
      (if (and _returnvalue_2 (== Component (`.HitComponent` (`GameplayStatics.BreakHitResult` _outhit))))
        (return true)
        (else
          (set `local.Theta` (+ (`local.Theta`) Resolution)))))
    (return false)
    (else
      (return false))))

(fn `GenerateIndices`
  (params (NumIndices :type Integer))
  (bind _indices (`self.Indices`))
  (`KismetArrayLibrary.Array_Clear` _indices)
  (for _index (range NumIndices)
    (`KismetArrayLibrary.Array_Add` _indices _index))
  (`KismetArrayLibrary.Array_RemoveItem` _indices (`self.CurrentMarker`))
  (return))

(fn `RandomMarker`
  (returns (Marker :type "StaticMeshComponent Object Reference"))
  (locals (RandomIndex :type Integer))
  (bind _nummarkers (`self.NumMarkers`))
  (`self.GenerateIndices` _nummarkers)
  (while (> (`KismetArrayLibrary.Array_Length` (`self.Indices`)) 0)
    (bind _output_get (set `local.RandomIndex` (`KismetMathLibrary.RandomInteger` _nummarkers)))
    (bind _output (`|GetArrayItem` (`self.Indices`) _output_get))
    (if (not (== (`self.CurrentMarker`) _output))
      (bind _output_get_2 (set `self.CurrentMarker` _output))
      (return (`|GetArrayItem` (`self.Markers`) _output_get_2))))
  (`KismetSystemLibrary.PrintString` "YOU DUN FUCKED UP BIG TIME")
  (return null))

(fn `SearchMarkers`
  (returns (Index :type Integer) (Found :type Boolean))
  (locals (RandomIndex :type Integer :default 0))
  (bind _indices (`self.Indices`))
  (bind _returnvalue (`KismetArrayLibrary.Array_Length` _indices))
  (`self.GenerateIndices` (`self.NumMarkers`))
  (while (> _returnvalue 0)
    (bind _output_get (set `local.RandomIndex` (`KismetMathLibrary.RandomInteger` _returnvalue)))
    (bind _output (`|GetArrayItem` _indices _output_get))
    (bind _isvisible (`self.ComponentIsVisible` (`|GetArrayItem` (`self.Markers`) _output) 30.0))
    (if _isvisible
      (`KismetArrayLibrary.Array_RemoveItem` _indices _output)
      (else
        (return _output true))))
  (return 0 false))

(fn `UserConstructionScript`)