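; Cyclic QWOB object that teleports between tagged markers when the player is not looking at it or blinks while watching it.
; Tick and blink events pick the next marker sequentially or randomly, unless locker or eye-state locks apply.
; Regular teleports require an unseen destination, tested against cached mesh vertices, and retry on a timer.
; A physics-capable marker carries the logic while the visual follows it, and movement clears the current marker index.
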(event `self.ReceiveBeginPlay`
  (bind _hidemarkers (`self.HideMarkers`))
  (bind _markers (`self.Markers`))
  ;[0 0 0] BeginPlay: Initialize Markers and Qwob
  (`|ExecutionSequence`
    (:`then_0`
      (bind _asbp_main_player (cast `/Game/Blueprints/BP_MainPlayer` (`GameplayStatics.GetPlayerPawn` 0)))
      (bind _output_get (set `self.PlayerREF` _asbp_main_player))
      (`self.AddTickPrerequisiteActor` _output_get)
      (add `/Game/Blueprints/BP_MainPlayer.FinishedInit` _output_get (`|CreateDelegate` :!event `Bind to Blink`)))
    (:`then_1`
      (`self.SortMarkers` (`self.GetComponentsByTag` "/Script/Engine.StaticMeshComponent" "MarkerTemp"))
      (set `self.NumMarkers` (`KismetArrayLibrary.Array_Length` _markers))
      (bind _output_get_2 (set `self.CurrentMarker` 0))
      (`self.GetVertices` _markers)
      (`self.UpdateQWOB` _output_get_2)
      (`self.InitTags`))
    (:`then_2`
      (`KismetSystemLibrary.K2_SetTimer` null "CheckForMovement" 0.1 true)
      (for _array_element (`self.Markers`)
        (`SceneComponent.SetHiddenInGame` _array_element _hidemarkers false))
      (`SceneComponent.SetHiddenInGame` (`self.QWOBMarker`) _hidemarkers false))))

(event `self.ReceiveTick`
  (params (DeltaSeconds :type "Float (single-precision)"))
  (bind _qwobtype (`self.QwobType`))
  (bind (_returnvalue_location _returnvalue_rotation) (`KismetMathLibrary.BreakTransform` (`SceneComponent.K2_GetComponentToWorld` (`self.QWOBMarker`))))
  ;[0 0 0] Event Tick: Check whether to update Qwob or not
  (`|ExecutionSequence`
    (:`then_0`
      (bind _locked (`self.CheckRegularLocks`))
      (if (not _locked)
        (bind _isvisible (`self.IsComponentVisible` (`self.QWOBMarker`)))
        (if _isvisible
          (set `self.HasUpdated` false)
          (`KismetSystemLibrary.K2_ClearAndInvalidateTimerHandle` (`self.TeleportTimerREF`))
          (elif (not (`self.HasUpdated`))
            (switch `/Game/Blueprints/Objects/ENUM_QwobType` _qwobtype :!label _label
              (:`NewEnumerator0`
                (bind (_index _found) (`self.SearchMarkersSequential` false)))
              (:`NewEnumerator1`
                (bind (_index_2 _found_2) (`self.SearchMarkersRandom` false))))
            (if (select `/Game/Blueprints/Objects/ENUM_QwobType` _qwobtype :`NewEnumerator0` _found :`NewEnumerator1` _found_2)
              (set `self.TryingToTeleport` false)
              (`self.UpdateQWOB` (select `/Game/Blueprints/Objects/ENUM_QwobType` _qwobtype :`NewEnumerator0` _index :`NewEnumerator1` _index_2))
              (else
                (bind _returnvalue (`KismetSystemLibrary.K2_SetTimerDelegate` (delegate `TryTeleport`) 0.1 true))
                (set `self.TeleportTimerREF` _returnvalue)
                (set `self.TryingToTeleport` true)))
            (set `self.HasUpdated` true)))))
    (:`then_1`
      (`SceneComponent.K2_SetWorldLocationAndRotation` (`self.QWOBVisual`) _returnvalue_location _returnvalue_rotation false false))))

(event `TryTeleport`
  ;[0 0 0] Event Tick: Check whether to update Qwob or not
  (goto _label))

(event `Blink`
  (bind _indices (`self.Indices`))
  ;[0 0 0] Blink behavior
  (bind _locked (`self.CheckBlinkLocks`))
  (if (not _locked)
    (bind _isvisible (`self.IsComponentVisible` (`self.QWOBMarker`)))
    (if _isvisible
      (`self.GenerateIndices` (`self.NumMarkers`) :!label _label_2)
      (`self.UpdateQWOB` (select `/Game/Blueprints/Objects/ENUM_QwobType` (`self.QwobType`) :`NewEnumerator0` (`|GetArrayItem` _indices) :`NewEnumerator1` (`KismetArrayLibrary.Array_Random` _indices)))
      (`self.ClosedEyes`)
      (set `self.HasUpdated` true)
      (elif (`self.TryingToTeleport`)
        (goto _label_2)))))

(event `/Game/Blueprints/BI_ObjectFunctionality.Emancipate`
  (bind _qwobmarker (`self.QWOBMarker`))
  (`PrimitiveComponent.SetSimulatePhysics` _qwobmarker false)
  (`SceneComponent.K2_AddWorldOffset` _qwobmarker (0.0 0.0 -1000.0) false true)
  (set `self.HasUpdated` false)
  (`KismetSystemLibrary.Delay` 0.5)
  (`PrimitiveComponent.SetSimulatePhysics` _qwobmarker true))

(event `/Game/Blueprints/BI_ObjectFunctionality.UpdateLock`
  (params (IsLocked :type Boolean))
  (set `self.IsInLocker` IsLocked))

(event `/Game/Blueprints/BI_ObjectFunctionality.UpdatePhysics`
  (params (On :type Boolean))
  (`PrimitiveComponent.SetSimulatePhysics` (`self.QWOBMarker`) On))

(event `Bind to Blink`
  (bind _blinkeffectwidget (`/Game/Blueprints/BP_MainPlayer.BlinkEffectWidget` (`self.PlayerREF`)))
  ;[0 0 0] Blink behavior
  (add `/Game/Blueprints/UI/BPW_BlinkEffect.EyesClosed` _blinkeffectwidget (`|CreateDelegate` :!event `Blink`))
  (add `/Game/Blueprints/UI/BPW_BlinkEffect.EyesOpened` _blinkeffectwidget (delegate `OpenedEyes`)))

(event `OpenedEyes`
  ;[0 0 0] Blink behavior
  (set `self.EyesIsClosed` false))

(event `ClosedEyes`
  ;[0 0 0] Blink behavior
  (set `self.EyesIsClosed` true))

(fn `CheckBlinkLocks`
  (returns (Locked :type Boolean))
  ;[0 0 0] Check if locked by Locker
  (if (`self.IsInLocker`)
    (return true)
    (else
      (return false))))

(fn `CheckForMovement`
  (if (> (`KismetMathLibrary.VSize` (`SceneComponent.GetComponentVelocity` (`self.QWOBMarker`))) (`self.MovementThreshold`))
    (set `self.CurrentMarker` -1)))

(fn `CheckRegularLocks`
  (returns (Locked :type Boolean))
  ;[0 0 0] Check if eyes are closed, or locked by a Locker
  (if (`self.EyesIsClosed`)
    (return true)
    (elif (`self.IsInLocker`)
      (return true)
      (else
        (return false)))))

(fn `GenerateIndices`
  (params (NumIndices :type Integer))
  (bind _indices (`self.Indices`))
  (bind _currentmarker (`self.CurrentMarker`))
  ;[0 0 0] Make integer array of element index
  (`KismetArrayLibrary.Array_Clear` _indices)
  (for _index (range 1 (+ NumIndices 1))
    (`KismetArrayLibrary.Array_Add` _indices (mod (+ _index _currentmarker) NumIndices)))
  (`KismetArrayLibrary.Array_RemoveItem` _indices _currentmarker)
  (return))

(fn `GetVertices`
  (params (Array :type "Array of StaticMeshComponent Object Reference"))
  (bind _output (`|GetArrayItem` Array))
  (bind _returnvalue (`KismetArrayLibrary.Array_Length` (`self.Vertices`)))
  ;[0 0 0] Stores vertices of mesh, removes duplicates. turns off tick if vertices exceeds max amount
  (bind _vertices (`KismetProceduralMeshLibrary.GetSectionFromStaticMesh` (`StaticMeshComponent.StaticMesh` _output)))
  (for _array_element _vertices
    (`KismetArrayLibrary.Array_AddUnique` (`self.Vertices`) (* _array_element (`SceneComponent.K2_GetComponentScale` _output))))
  (if (> _returnvalue 100)
    (`self.SetActorTickEnabled` false)
    (`KismetSystemLibrary.PrintString` (`KismetStringLibrary.Concat_StrStr` "Too many vertices in QWOB mesh: " (`KismetStringLibrary.Conv_IntToString` _returnvalue)) true true (struct :`G` 0.66 :`B` 1.0 :`A` 1.0) 5.0)))

(fn `InitTags`
  (bind _tags (`/Game/Blueprints/BPL_VisibilityAndTagging.MakeTags` (`|MakeArray` "NewEnumerator2" :!type "/Game/Blueprints/ENUM_Tags Enum")))
  (set `ActorComponent.ComponentTags` _tags (`self.QWOBVisual`))
  (bind _tags_2 (`/Game/Blueprints/BPL_VisibilityAndTagging.MakeTags` (select `bool` (`self.EffectsPressurePlates`) :`false` (`|MakeArray` "NewEnumerator1" :!type "/Game/Blueprints/ENUM_Tags Enum") :`true` (`|MakeArray` "NewEnumerator1" "NewEnumerator3" :!type "/Game/Blueprints/ENUM_Tags Enum"))))
  (set `ActorComponent.ComponentTags` _tags_2 (`self.QWOBMarker`))
  (for _array_element (`self.Markers`)
    (bind _tags_3 (`/Game/Blueprints/BPL_VisibilityAndTagging.MakeTags` (`|MakeArray` "NewEnumerator0" :!type "/Game/Blueprints/ENUM_Tags Enum")))
    (set `ActorComponent.ComponentTags` _tags_3 _array_element)))

(fn `IsComponentVisible`
  (params (Component :type "StaticMeshComponent Object Reference"))
  (returns (IsVisible :type Boolean))
  (bind _component (`local.Component`))
  (for _array_element (`/Game/Blueprints/BP_MainPlayer.VisibleQwobs` (`self.PlayerREF`))
    (if (== _array_element _component)
      (return true)))
  (bind _isvisible (`/Game/Blueprints/BPL_VisibilityAndTagging.Is Component Visible` (`self.Vertices`) _component))
  (if _isvisible
    (return true)
    (else
      (return false))))

(fn `SearchMarkersRandom`
  (params (SearchForVisible :type Boolean))
  (returns (Index :type Integer) (Found :type Boolean))
  (locals (CurrentIndex :type Integer :default 0))
  (bind _indices (`self.Indices`))
  (bind _returnvalue (`KismetArrayLibrary.Array_Length` _indices))
  (bind _output (`|GetArrayItem` _indices (`KismetMathLibrary.RandomInteger` _returnvalue)))
  ;[0 0 0] Search through all markers, return any not visible if any
  (`self.GenerateIndices` (`self.NumMarkers`))
  (while (> _returnvalue 0)
    (bind _isvisible (`self.IsComponentVisible` (`|GetArrayItem` (`self.Markers`) _output)))
    (if (select `bool` (`local.SearchForVisible`) :`false` _isvisible :`true` (not _isvisible))
      (`KismetArrayLibrary.Array_RemoveItem` _indices _output)
      (else
        (return _output true))))
  (return 0 false))

(fn `SearchMarkersSequential`
  (params (SearchForVisible :type Boolean))
  (returns (Index :type Integer) (Found :type Boolean))
  (locals (CurrentIndex :type Integer :default 0))
  ;[0 0 0] Search through all markers, return any not visible if any
  (`self.GenerateIndices` (`self.NumMarkers`))
  (for _array_element (`self.Indices`)
    (bind _isvisible (`self.IsComponentVisible` (`|GetArrayItem` (`self.Markers`) _array_element)))
    (if (not (select `bool` (`local.SearchForVisible`) :`false` _isvisible :`true` (not _isvisible)))
      (return _array_element true)))
  (return 0 false))

(fn `SortMarkers`
  (params (UnsortedMarkers :type "Array of StaticMeshComponent Object Reference"))
  (locals (SortedTemp :type "Array of StaticMeshComponent Object Reference"))
  (bind _sortedtemp (`local.SortedTemp`))
  (bind _markers (`self.Markers`))
  (`KismetArrayLibrary.Array_Clear` _sortedtemp)
  (for _array_element UnsortedMarkers
    (bind _returnvalue (`KismetSystemLibrary.GetDisplayName` _array_element))
    (`KismetArrayLibrary.Array_Set` (`local.SortedTemp`) (`KismetStringLibrary.Conv_StringToInt` (`KismetStringLibrary.Split` (`KismetStringLibrary.RightChop` _returnvalue (+ (`KismetStringLibrary.FindSubstring` _returnvalue "Marker" false true) 6)) " ")) _array_element true))
  (`KismetArrayLibrary.Array_Clear` _markers)
  (for (_array_element_2 _array_index) _sortedtemp
    (`KismetArrayLibrary.Array_Set` _markers _array_index _array_element_2 true))
  (return))

(fn `UpdateQWOB`
  (params (Marker :type Integer))
  (bind _charactermovement (`Character.CharacterMovement` (`self.PlayerREF`)))
  ;[0 0 0] Teleports Qwob to selected marker
  (bind _output_get (set `self.CurrentMarker` Marker))
  (if (not (`self.CanTeleportPlayer`))
    (`CharacterMovementComponent.SetMovementMode` _charactermovement "MOVE_Custom" 0))
  (`GameplayStatics.PlaySoundAtLocation` (`self.TeleportSFX`) (`SceneComponent.K2_GetComponentLocation` (`self.QWOBMarker`)) (struct) 1.5 1.0 0.0 "/Game/FPSPuzzleSP/Blueprints/Components/SoundAttenuation.SoundAttenuation" null null null)
  (bind (_returnvalue_location _returnvalue_rotation _returnvalue_scale) (`KismetMathLibrary.BreakTransform` (`SceneComponent.K2_GetComponentToWorld` (`|GetArrayItem` (`self.Markers`) _output_get))))
  (`SceneComponent.K2_SetWorldTransform` (`self.QWOBMarker`) (`KismetMathLibrary.MakeTransform` _returnvalue_location _returnvalue_rotation _returnvalue_scale) false true)
  (`CharacterMovementComponent.SetMovementMode` _charactermovement "MOVE_Walking" 0)
  (`KismetSystemLibrary.K2_ClearAndInvalidateTimerHandle` (`self.TeleportTimerREF`)))

(fn `UserConstructionScript`)