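; Level-streaming trigger actor that swaps sublevels once its transition object becomes visible to the player.
; The player's first overlap of the activation trigger enables Tick, which checks the player's VisibleQwobs list, then tests visibility using scaled mesh vertices cached at BeginPlay.
; On first sighting it unloads LevelFrom, loads LevelTo and plays a sound.
; Once out of view, it hides the object, destroys its light, re-materials the light mesh and stops ticking.
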(event `self.ReceiveBeginPlay`
  (bind _transitionobject (`self.TransitionObject`))
  (bind _vertices (`KismetProceduralMeshLibrary.GetSectionFromStaticMesh` (`StaticMeshComponent.StaticMesh` _transitionobject)))
  (for _array_element _vertices
    (`KismetArrayLibrary.Array_AddUnique` (`self.Vertices`) (* _array_element (`SceneComponent.K2_GetComponentScale` _transitionobject)))))

(event `self.ReceiveTick`
  (params (DeltaSeconds :type "Float (single-precision)"))
  (bind _lightmesh (`self.LightMesh`))
  (bind _levelto (`self.LevelTo`))
  (bind _levelfrom (`self.LevelFrom`))
  (bind _safeload (`self.SafeLoad`))
  (if (`self.HasSwitched`)
    (bind _isvisible (`self.IsTransitionVisible`))
    (if (not _isvisible)
      (`SceneComponent.SetHiddenInGame` (`self.TransitionObject`) true true)
      (`self.SetActorTickEnabled` false)
      (`self.K2_DestroyActor` (`self.Light`))
      (`/Engine/EditorBlueprintResources/StandardMacros.IsValid` _lightmesh
        (:`Is Valid`
          (`PrimitiveComponent.CreateDynamicMaterialInstance` (`StaticMeshActor.StaticMeshComponent` _lightmesh) 1 "/Game/StarterContent/Materials/M_Metal_Burnished_Steel.M_Metal_Burnished_Steel" "None"))))
    (else
      (bind _isvisible_2 (`self.IsTransitionVisible`))
      (if _isvisible_2
        (set `self.HasSwitched` true)
        (if (not (`KismetStringLibrary.IsEmpty` _levelfrom))
          (`GameplayStatics.UnloadStreamLevel` (`KismetStringLibrary.Conv_StringToName` _levelfrom) _safeload))
        (if (`KismetStringLibrary.IsEmpty` _levelto)
          (`KismetSystemLibrary.PrintString` "No level to load specified")
          (else
            (`GameplayStatics.LoadStreamLevel` (`KismetStringLibrary.Conv_StringToName` _levelto) true _safeload)
            (`GameplayStatics.PlaySoundAtLocation` (`self.LoadInSFX`) (`SceneComponent.K2_GetComponentLocation` (`self.TransitionObject`)) (struct) 1.0 1.0 0.0 null null null null)))))))

(event `self.ActivationTrigger.OnComponentBeginOverlap`
  (params (OverlappedComponent :type "PrimitiveComponent Object Reference") (OtherActor :type "Actor Object Reference") (OtherComp :type "PrimitiveComponent Object Reference") (OtherBodyIndex :type Integer) (bFromSweep :type Boolean) (SweepResult :type "HitResult Structure (by ref)"))
  (bind _asbp_main_player (cast `/Game/Blueprints/BP_MainPlayer` OtherActor))
  (`/Engine/EditorBlueprintResources/StandardMacros.DoOnce` false
    (:`Completed`
      (set `self.PlayerREF` _asbp_main_player)
      (`self.SetActorTickEnabled` true))))

(fn `IsTransitionVisible`
  (returns (IsVisible :type Boolean))
  (bind _transitionobject (`self.TransitionObject`))
  (for _array_element (`/Game/Blueprints/BP_MainPlayer.VisibleQwobs` (`self.PlayerREF`))
    (if (== _array_element _transitionobject)
      (return true)))
  (bind _isvisible (`/Game/Blueprints/BPL_VisibilityAndTagging.Is Component Visible` (`self.Vertices`) _transitionobject))
  (if _isvisible
    (return true)
    (else
      (return false))))

(fn `UserConstructionScript`)