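; BP_QwobReceptor is an unfinished receptor object that detects nearby Qwobs, identified by a tagged static mesh component on the overlapping actor.
; Its sphere overlaps maintain a list of those actors and set an overlap flag, which is never cleared here.
; At BeginPlay it binds to the player's grab and ungrab events, but the Grab and Ungrab responses are empty.
; The tag-setup logic is disconnected.
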(event `Ungrab`
  (if (`self.HasOverlap`)
    _))

(event `self.ReceiveBeginPlay`
  (`|ExecutionSequence`
    (:`then_0`
      (bind _asbp_main_player (cast `/Game/Blueprints/BP_MainPlayer` (`GameplayStatics.GetPlayerCharacter` 0)))
      (bind _output_get (set `self.PlayerREF` _asbp_main_player))
      (add `/Game/Blueprints/BP_MainPlayer.Ungrabbed` _output_get (`|CreateDelegate` :!event `Ungrab`))
      (add `/Game/Blueprints/BP_MainPlayer.Grabbed` _output_get (`|CreateDelegate` :!event `Grab`)))))

(event `Grab`)

(event `self.Sphere.OnComponentBeginOverlap`
  (params (OverlappedComponent :type "PrimitiveComponent Object Reference") (OtherActor :type "Actor Object Reference") (OtherComp :type "PrimitiveComponent Object Reference") (OtherBodyIndex :type Integer) (bFromSweep :type Boolean) (SweepResult :type "HitResult Structure (by ref)"))
  (`/Engine/EditorBlueprintResources/StandardMacros.IsValid` (`|GetArrayItem` (`self.GetComponentsByTag` OtherActor "/Script/Engine.StaticMeshComponent" (`self.TagtoCheck`)))
    (:`Is Valid`
      (`KismetArrayLibrary.Array_AddUnique` (`self.OverlappingQwobs`) OtherActor)
      (set `self.HasOverlap` true))))

(event `self.Sphere.OnComponentEndOverlap`
  (params (OverlappedComponent :type "PrimitiveComponent Object Reference") (OtherActor :type "Actor Object Reference") (OtherComp :type "PrimitiveComponent Object Reference") (OtherBodyIndex :type Integer))
  (bind _overlappingqwobs (`self.OverlappingQwobs`))
  (for _array_element _overlappingqwobs
    (if (== _array_element OtherActor)
      (`KismetArrayLibrary.Array_RemoveItem` _overlappingqwobs OtherActor)
      (break)))
  (if (== (`KismetArrayLibrary.Array_Length` _overlappingqwobs) 0)
    _))

(fn `UserConstructionScript`)