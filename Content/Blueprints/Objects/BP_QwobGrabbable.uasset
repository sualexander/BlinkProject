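; BP_QwobGrabbable is a grabbable QWOB object, a child Blueprint that adds grab handling and lock rules to its parent.
; Interact toggles grab state and the QWOBMarker collision type, clearing the current marker and playing a sound on pickup.
; Lock checks report locked while grabbed or in a Locker, with closed eyes also counting outside the blink check.
; Emancipate teleports the marker upward with physics briefly disabled, and a visibility check tests QWOBMarker.
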(event `self.ReceiveBeginPlay`
  ;[0 0 0] BeginPlay: Bind to GrabComponent event dispatcher
  (`parent.ReceiveBeginPlay`))

(event `self.ReceiveTick`
  (params (DeltaSeconds :type "Float (single-precision)"))
  ;[0 0 0] BeginPlay: Bind to GrabComponent event dispatcher
  (`parent.ReceiveTick` DeltaSeconds))

(event `/Game/Blueprints/BI_Interact.Interact`
  (params (WasGrabbing :type Boolean))
  (bind _qwobmarker (`self.QWOBMarker`))
  (if WasGrabbing
    (`PrimitiveComponent.SetCollisionObjectType` _qwobmarker "ECC_WorldStatic")
    (set `self.IsGrabbing` false)
    (else
      (set `self.CurrentMarker` -1)
      (`PrimitiveComponent.SetCollisionObjectType` _qwobmarker "ECC_WorldDynamic")
      (set `self.IsGrabbing` true)
      (`self.OnGrab`)
      (`GameplayStatics.PlaySound2D` "/Game/_Sound/SFX/Grab_Cue.Grab_Cue" 1.0 1.0 0.0 null null))))

(event `/Game/Blueprints/BI_Interact.Emancipate`
  (`PrimitiveComponent.SetSimulatePhysics` (`self.QWOBMarker`) false)
  (`SceneComponent.K2_AddWorldOffset` (`self.QWOBMarker`) (0.0 0.0 1000.0) false true)
  (`KismetSystemLibrary.Delay` 0.5)
  (`PrimitiveComponent.SetSimulatePhysics` (`self.QWOBMarker`) true))

(fn `CheckBlinkLocks`
  (returns (Locked :type Boolean))
  ;[0 0 0] Check if grabbing, or locked by Locker
  (if (`self.IsGrabbing`)
    (return true)
    (elif (`self.IsInLocker`)
      (return true)
      (else
        (return false)))))

(fn `CheckRegularLocks`
  (returns (Locked :type Boolean))
  ;[0 0 0] Check if currently grabbing, or eyes are closed, or locked by a Locker
  (if (`self.IsGrabbing`)
    (return true)
    (elif (`self.EyesClosed`)
      (return true)
      (elif (`self.IsInLocker`)
        (return true)
        (else
          (return false))))))

(fn `ToObjectRaycast`
  (returns (IsVisible :type Boolean))
  ;[0 0 0] Call visibility function on Qwob
  (bind _isvisible (`/Game/Blueprints/BPL_VisibilityFunctions.Is Component Visible` (`self.Vertices`) (`self.QWOBMarker`)))
  (return _isvisible))

(fn `UserConstructionScript`
  (`parent.UserConstructionScript`))