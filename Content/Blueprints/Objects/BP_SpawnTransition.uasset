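; BP_SpawnTransition is an object that moves the game to another level once an object raycast check succeeds.
; FinalAction starts a fast looping timer that polls ToObjectRaycast.
; The first success passes a DoOnce, clears the timer and, after a short delay, opens Level1 by object reference.
; BeginPlay, overlap and Tick only call their parent versions.
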(event `self.ReceiveBeginPlay`
  (`parent.ReceiveBeginPlay`))

(event `self.ReceiveActorBeginOverlap`
  (params (OtherActor :type "Actor Object Reference"))
  (`parent.ReceiveActorBeginOverlap` OtherActor))

(event `self.ReceiveTick`
  (params (DeltaSeconds :type "Float (single-precision)"))
  (`parent.ReceiveTick` DeltaSeconds))

(event `self.FinalAction`
  (bind _returnvalue (`KismetSystemLibrary.K2_SetTimerDelegate` (delegate `TeleportTimer`) 0.1 true))
  (bind _output_get (set `self.TimerREF` _returnvalue)))

(event `TeleportTimer`
  (bind _isvisible (`self.ToObjectRaycast`))
  (if _isvisible
    (`/Engine/EditorBlueprintResources/StandardMacros.DoOnce` false
      (:`Completed`
        (`KismetSystemLibrary.K2_ClearAndInvalidateTimerHandle` (stale `self.FinalAction` _output_get))
        (`KismetSystemLibrary.Delay` 0.5)
        (`GameplayStatics.OpenLevelBySoftObjectPtr` "/Game/Levels/Level1.Level1")))))

(fn `UserConstructionScript`
  (`parent.UserConstructionScript`))