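; Grabbable QWOB object that can be picked up and moved among markers, extending a parent class's behavior.
; Interact toggles grabbing, clearing the current marker and calling OnGrab on pickup, while Emancipate sends the QWOB to a random marker index.
; Lock checks report locked while grabbed or in a Locker; the regular check also counts closed eyes, unlike the blink check.
; A vertex-based visibility test serves as the object raycast.
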(event `self.ReceiveBeginPlay`
  ;[0 0 0] BeginPlay: Bind to GrabComponent event dispatcher
  (`parent.ReceiveBeginPlay`))

(event `self.ReceiveTick`
  (params (DeltaSeconds :type "Float (single-precision)"))
  ;[0 0 0] BeginPlay: Bind to GrabComponent event dispatcher
  (`parent.ReceiveTick` DeltaSeconds))

(event `/Game/Blueprints/BI_Interact.Interact`
  (params (WasGrabbing :type Boolean))
  (if WasGrabbing
    (set `self.IsGrabbing` false)
    (else
      (set `self.CurrentMarker` -1)
      (set `self.IsGrabbing` true)
      (`self.OnGrab`))))

(event `/Game/Blueprints/BI_Interact.Emancipate`
  (`self.GenerateIndices` (`self.NumMarkers`))
  (`self.UpdateQWOB` (`KismetArrayLibrary.Array_Random` (`self.Indices`))))

(fn `CheckBlinkLocks`
  (returns (Locked :type Boolean))
  ;[0 0 0] Check if grabbing, or locked by Locker
  (if (`self.IsGrabbing`)
    (return true)
    (elif (`self.IsInLocker`)
      (return true)
      (else
        (return false)))))

(fn `CheckRegularLocks`
  (returns (Locked :type Boolean))
  ;[0 0 0] Check if currently grabbing, or eyes are closed, or locked by a Locker
  (if (`self.IsGrabbing`)
    (return true)
    (elif (`self.EyesClosed`)
      (return true)
      (elif (`self.IsInLocker`)
        (return true)
        (else
          (return false))))))

(fn `ToObjectRaycast`
  (returns (IsVisible :type Boolean))
  ;[0 0 0] Call visibility function on Qwob
  (bind _isvisible (`/Game/Blueprints/VisibilityFunctions.Is Component Visible` (`self.Vertices`) (`self.QWOB`)))
  (return _isvisible))

(fn `UserConstructionScript`
  (`parent.UserConstructionScript`))