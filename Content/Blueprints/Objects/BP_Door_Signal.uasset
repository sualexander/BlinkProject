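; BP_Door_Signal is a signal-controlled door that teleports the player to its Marker when hit while active.
; Turn events raise or lower a signal count, activating the door at SignalThreshold and deactivating it below.
; Activation state tints a dynamic material on the Cube green or white, starting inactive, and prints a debug message.
; Cube hits from BP_MainPlayer pass through a DoOnce that resets after a short delay, preventing repeated teleports.
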(event `self.ReceiveBeginPlay`
  (bind _returnvalue (`PrimitiveComponent.CreateDynamicMaterialInstance` (`self.Cube`) 0 "/Game/Materials/MI_SingularLaser.MI_SingularLaser" "None"))
  (set `self.Material` _returnvalue)
  (`self.Deactivate`))

(event `Activate`
  (`MaterialInstanceDynamic.SetVectorParameterValue` (`self.Material`) "Color" (struct :`R` 0.384314 :`G` 1.0 :`B` 0.32549 :`A` 1.0))
  (set `self.IsActive` true)
  (`KismetSystemLibrary.PrintString` "Door activate"))

(event `Deactivate`
  (`MaterialInstanceDynamic.SetVectorParameterValue` (`self.Material`) "Color" (struct :`R` 1.0 :`G` 1.0 :`B` 1.0 :`A` 1.0))
  (set `self.IsActive` false)
  (`KismetSystemLibrary.PrintString` "Door deactivate"))

(event `self.Cube.OnComponentHit`
  (params (HitComponent :type "PrimitiveComponent Object Reference") (OtherActor :type "Actor Object Reference") (OtherComp :type "PrimitiveComponent Object Reference") (NormalImpulse :type "Vector Structure") (Hit :type "HitResult Structure (by ref)"))
  (if (`self.IsActive`)
    (if (== (`GameplayStatics.GetObjectClass` OtherActor) "/Game/Blueprints/BP_MainPlayer.BP_MainPlayer_C")
      (`/Engine/EditorBlueprintResources/StandardMacros.DoOnce` false :!label _label
        (:`Completed`
          (`self.K2_SetActorLocation` (`GameplayStatics.GetPlayerPawn` 0) (`SceneComponent.K2_GetComponentLocation` (`self.Marker`)) false false)
          (`KismetSystemLibrary.Delay` 1.0)
          (goto _label :!via `Reset`))))))

(event `/Game/FPSPuzzleSP/Blueprints/Components/BI_Signal.Turn`
  (params (Signal :type "/Game/FPSPuzzleSP/Blueprints/Components/Enum_Signal Enum" :default "NewEnumerator0"))
  (bind _totalsignals (`self.totalSignals`))
  (bind _isactive (`self.IsActive`))
  (switch `/Game/FPSPuzzleSP/Blueprints/Components/Enum_Signal` Signal
    (:`NewEnumerator0`
      (`/Engine/EditorBlueprintResources/StandardMacros.IncrementInt` _totalsignals
        (:`  `
          _)))
    (:`NewEnumerator1`
      (`/Engine/EditorBlueprintResources/StandardMacros.DecrementInt` _totalsignals
        (:`  `
          _))))
  (if (>= (`self.totalSignals`) (`self.SignalThreshold`))
    (if (not _isactive)
      (`self.Activate`))
    (elif _isactive
      (`self.Deactivate`))))

(fn `NewFunction`)

(fn `UserConstructionScript`)