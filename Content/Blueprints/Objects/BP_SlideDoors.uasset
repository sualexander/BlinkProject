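; Signal-driven door that opens by dissolving its material, dropping collision and hiding its mesh, despite the SlideDoors name.
; Turn opens or closes it directly, or counts On/Off signals against SignalThreshold when that exceeds one.
; Open and Close play a sound, relay optionally inverted signals to Outputs, and run the dissolve timeline forward or backward.
; Turn also recolors linked Lights and Meshes to OnColor or white.
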(event `PlaySound`
  (params (IsOpen :type Boolean))
  (bind _returnvalue (`SceneComponent.K2_GetComponentLocation` (`self.StaticMesh`)))
  (if IsOpen
    (`GameplayStatics.PlaySoundAtLocation` "/Engine/EditorSounds/Notifications/CompileFailed.CompileFailed" _returnvalue (struct) 1.0 1.0 0.0 null null null null)
    (else
      (`GameplayStatics.PlaySoundAtLocation` "/Engine/EditorSounds/GamePreview/EjectFromPlayer.EjectFromPlayer" _returnvalue (struct) 1.0 1.0 0.0 null null null null))))

(event `self.ReceiveBeginPlay`
  (bind _returnvalue (`PrimitiveComponent.CreateDynamicMaterialInstance` (`self.StaticMesh`) 0 "/Game/Materials/Area1/MI_Level1Door.MI_Level1Door" "None"))
  (set `self.DoorMaterial` _returnvalue))

(event `Open`
  (bind _staticmesh (`self.StaticMesh`))
  (set `self.IsOpen` true)
  (for _array_element (`self.Outputs`)
    (message `/Game/Blueprints/BI_Signal.Turn` _array_element (select `bool` (`self.InverseSignals`) :`false` "NewEnumerator0" :`true` "NewEnumerator1" :!type "/Game/FPSPuzzleSP/Blueprints/Components/Enum_Signal Enum")))
  (`PrimitiveComponent.SetCollisionEnabled` _staticmesh "NoCollision")
  (`self.PlaySound` false)
  (bind (_direction _track) (`Timeline|TL_Open` :!label _label)
    (:`Update`
      (`MaterialInstanceDynamic.SetScalarParameterValue` (`self.DoorMaterial`) "Dissolve" _track))
    (:`Finished`
      (if (`self.IsOpen`)
        (`SceneComponent.SetHiddenInGame` _staticmesh true false)))))

(event `Close`
  (bind _staticmesh (`self.StaticMesh`))
  (set `self.IsOpen` false)
  (for _array_element (`self.Outputs`)
    (message `/Game/Blueprints/BI_Signal.Turn` _array_element (select `bool` (`self.InverseSignals`) :`false` "NewEnumerator1" :`true` "NewEnumerator0" :!type "/Game/FPSPuzzleSP/Blueprints/Components/Enum_Signal Enum")))
  (`SceneComponent.SetHiddenInGame` _staticmesh false false)
  (`PrimitiveComponent.SetCollisionEnabled` _staticmesh "QueryAndPhysics")
  (`self.PlaySound` true)
  (goto _label :!via `Reverse`))

(event `/Game/Blueprints/BI_Signal.Turn`
  (params (Signal :type "/Game/FPSPuzzleSP/Blueprints/Components/Enum_Signal Enum" :default "NewEnumerator0"))
  (bind _totalsignals (`self.TotalSignals`))
  (bind _isopen (`self.IsOpen`))
  (if (<= (`self.SignalThreshold`) 1)
    (switch `/Game/FPSPuzzleSP/Blueprints/Components/Enum_Signal` Signal
      (:`NewEnumerator0`
        (`self.Open` :!label _label_2)
        (for _array_element (`self.Lights`)
          (`LightComponent.SetLightColor` (`Light.LightComponent` _array_element) (`self.OnColor`) true)
          (for _array_element_2 (`self.Meshes`)
            (bind _returnvalue (`PrimitiveComponent.CreateDynamicMaterialInstance` (`self.GetComponentByClass` _array_element_2 "/Script/Engine.StaticMeshComponent") (`self.MaterialIndex`) "/Game/Materials/MI_FakeWalls.MI_FakeWalls" "None"))
            (`MaterialInstanceDynamic.SetVectorParameterValue` _returnvalue "Color" (`self.OnColor`)))))
      (:`NewEnumerator1`
        (`self.Close` :!label _label_3)
        (for _array_element_3 (`self.Lights`)
          (`LightComponent.SetLightColor` (`Light.LightComponent` _array_element_3) (struct :`R` 1.0 :`G` 1.0 :`B` 1.0 :`A` 1.0) true)
          (for _array_element_4 (`self.Meshes`)
            (bind _returnvalue_2 (`PrimitiveComponent.CreateDynamicMaterialInstance` (`self.GetComponentByClass` _array_element_4 "/Script/Engine.StaticMeshComponent") (`self.MaterialIndex`) "/Game/Materials/MI_FakeWalls.MI_FakeWalls" "None"))
            (`MaterialInstanceDynamic.SetVectorParameterValue` _returnvalue_2 "Color" (struct :`R` 1.0 :`G` 1.0 :`B` 1.0 :`A` 1.0))))))
    (else
      (switch `/Game/FPSPuzzleSP/Blueprints/Components/Enum_Signal` Signal
        (:`NewEnumerator0`
          (`/Engine/EditorBlueprintResources/StandardMacros.IncrementInt` _totalsignals
            (:`  `
              _)))
        (:`NewEnumerator1`
          (`/Engine/EditorBlueprintResources/StandardMacros.DecrementInt` _totalsignals
            (:`  `
              _))))
      (if (>= _totalsignals (`self.SignalThreshold`))
        (if (not _isopen)
          (goto _label_2))
        (elif _isopen
          (goto _label_3))))))

(fn `UserConstructionScript`)