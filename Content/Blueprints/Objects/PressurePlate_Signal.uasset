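; Pressure plate that signals linked objects when a BP_QwobCyclic actor enters or leaves its trigger.
; On overlap it sets IsActive and tints a dynamic material with that actor's color; on exit it clears the flag and turns black.
; Both events send TurnMessage to every entry in Outputs.
; InverseSignals only affects the exit message, making it match the enter message, so it does not truly invert the signal.
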(event `self.ReceiveBeginPlay`
  (bind _returnvalue (`PrimitiveComponent.CreateDynamicMaterialInstance` (`self.StaticMesh`) 0 "/Game/Materials/M_PressurePlate.M_PressurePlate" "None"))
  (set `self.Mat0` _returnvalue))

(event `self.Trigger.OnComponentBeginOverlap`
  (params (OverlappedComponent :type "PrimitiveComponent Object Reference") (OtherActor :type "Actor Object Reference") (OtherComp :type "PrimitiveComponent Object Reference") (OtherBodyIndex :type Integer) (bFromSweep :type Boolean) (SweepResult :type "HitResult Structure (by ref)"))
  (bind _asbp_qwob_cyclic (cast `/Game/Blueprints/Objects/BP_QwobCyclic` OtherActor))
  (set `self.IsActive` true)
  (`MaterialInstanceDynamic.SetVectorParameterValue` (`self.Mat0`) "Color" (`/Game/Blueprints/Objects/BP_QwobCyclic.Color` _asbp_qwob_cyclic))
  (for _array_element (`self.Outputs`)
    (message `/Game/Blueprints/BI_Signal.Turn` _array_element (select `bool` (`self.Inverse signals`) :`false` "NewEnumerator0" :`true` "NewEnumerator0" :!type "/Game/FPSPuzzleSP/Blueprints/Components/Enum_Signal Enum"))))

(event `self.Trigger.OnComponentEndOverlap`
  (params (OverlappedComponent :type "PrimitiveComponent Object Reference") (OtherActor :type "Actor Object Reference") (OtherComp :type "PrimitiveComponent Object Reference") (OtherBodyIndex :type Integer))
  (cast `/Game/Blueprints/Objects/BP_QwobCyclic` OtherActor)
  (set `self.IsActive` false)
  (`MaterialInstanceDynamic.SetVectorParameterValue` :`self` (`self.Mat0`) :`ParameterName` "Color")
  (for _array_element (`self.Outputs`)
    (message `/Game/Blueprints/BI_Signal.Turn` _array_element (select `bool` (`self.Inverse signals`) :`false` "NewEnumerator1" :`true` "NewEnumerator0" :!type "/Game/FPSPuzzleSP/Blueprints/Components/Enum_Signal Enum"))))

(fn `UserConstructionScript`)