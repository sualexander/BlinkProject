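; Pressure plate that switches active when an actor tagged "Signals" overlaps its box, or is already overlapping shortly after BeginPlay.
; Activation sends a TurnMessage to each target in Outputs, with the value flipped for entries marked InvertSignal.
; A tagged actor leaving clears the active state without messaging outputs or checking for remaining occupants.
; UpdateOverlap only prints the state for debugging.
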(event `self.ReceiveBeginPlay`
  (`KismetSystemLibrary.Delay` 0.5)
  (bind _hasinitialoverlap (`self.CheckInitiallyOverlapping`))
  (if _hasinitialoverlap
    (set `self.IsActive` true :!label _label)
    (for _array_element (`self.Outputs`)
      (message `/Game/Blueprints/BI_Signal.Turn` (break `/Game/Blueprints/STRUCT_Signals` _array_element) (select `bool` (`.InvertSignal_5_DAF274A9474CC75ECB928ABBDE614AD0` (break `/Game/Blueprints/STRUCT_Signals` _array_element)) :`false` "NewEnumerator1" :`true` "NewEnumerator0" :!type "/Game/FPSPuzzleSP/Blueprints/Components/Enum_Signal Enum")))
    (`self.UpdateOverlap` (stale `self.Box.OnComponentEndOverlap` _output_get) :!label _label_2)
    (else
      (`KismetSystemLibrary.PrintString` "No Initial Overlap"))))

(event `self.Box.OnComponentBeginOverlap`
  (params (OverlappedComponent :type "PrimitiveComponent Object Reference") (OtherActor :type "Actor Object Reference") (OtherComp :type "PrimitiveComponent Object Reference") (OtherBodyIndex :type Integer) (bFromSweep :type Boolean) (SweepResult :type "HitResult Structure (by ref)"))
  (if (`self.IsActive`)
    _
    (elif (`self.ActorHasTag` OtherActor "Signals")
      (goto _label))))

(event `self.Box.OnComponentEndOverlap`
  (params (OverlappedComponent :type "PrimitiveComponent Object Reference") (OtherActor :type "Actor Object Reference") (OtherComp :type "PrimitiveComponent Object Reference") (OtherBodyIndex :type Integer))
  (if (`self.IsActive`)
    (if (`self.ActorHasTag` OtherActor "Signals")
      (bind _output_get (set `self.IsActive` false))
      (goto _label_2))))

(fn `CheckInitiallyOverlapping`
  (returns (HasInitialOverlap :type Boolean))
  (bind _overlappingactors (`self.GetOverlappingActors` "/Script/Engine.Actor"))
  (if (> (`KismetArrayLibrary.Array_Length` _overlappingactors) 0)
    (for _array_element _overlappingactors
      (if (`self.ActorHasTag` _array_element "Signals")
        (return true))))
  (return false))

(fn `UpdateOverlap`
  (params (IsOn :type Boolean))
  (`KismetSystemLibrary.PrintString` (`KismetStringLibrary.Conv_BoolToString` IsOn)))

(fn `UserConstructionScript`)