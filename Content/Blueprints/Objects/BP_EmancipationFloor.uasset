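; BP_EmancipationFloor is a trigger floor that emancipates tagged objects entering its box.
; On BeginPlay it builds the tag to match from an enum value and caches the player as BP_MainPlayer.
; On overlap, an actor with a static mesh component carrying that tag receives EmancipateMessage.
; If the player is grabbing anything at that moment, a forced ungrab runs first, without checking which object is held.
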(event `self.ReceiveBeginPlay`
  (bind _tags (`/Game/Blueprints/BPL_VisibilityAndTagging.MakeTags` (`|MakeArray` "NewEnumerator1" :!type "/Game/Blueprints/ENUM_Tags Enum")))
  (set `self.TagToCheck` (`|GetArrayItem` _tags))
  (bind _asbp_main_player (cast `/Game/Blueprints/BP_MainPlayer` (`GameplayStatics.GetPlayerCharacter` 0)))
  (set `self.PlayerREF` _asbp_main_player))

(event `self.Box.OnComponentBeginOverlap`
  (params (OverlappedComponent :type "PrimitiveComponent Object Reference") (OtherActor :type "Actor Object Reference") (OtherComp :type "PrimitiveComponent Object Reference") (OtherBodyIndex :type Integer) (bFromSweep :type Boolean) (SweepResult :type "HitResult Structure (by ref)"))
  (bind _playerref (`self.PlayerREF`))
  (if (> (`KismetArrayLibrary.Array_Length` (`self.GetComponentsByTag` OtherActor "/Script/Engine.StaticMeshComponent" (`self.TagToCheck`))) 0)
    (if (`/Game/Blueprints/BP_MainPlayer.IsGrabbing` _playerref)
      (`/Game/Blueprints/BP_MainPlayer.ForcedUngrab` _playerref))
    (message `/Game/Blueprints/BI_ObjectFunctionality.Emancipate` OtherActor)))

(fn `UserConstructionScript`)