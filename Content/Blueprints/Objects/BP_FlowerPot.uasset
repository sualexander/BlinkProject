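; BP_FlowerPot is a grabbable flower pot object that attaches to the player's camera and swaps to a Geometry Collection.
; BPGrabComponent triggers UpdateGrab: when IsGrabbing is false, the regular mesh attaches to the cached player's camera.
; When true, the mesh detaches and is destroyed, and a scaled FlowerPot Geometry Collection spawns at its location.
; Disconnected physics, delay and Chaos break-event nodes never run.
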(event `self.ReceiveBeginPlay`
  (add `/Game/Blueprints/BP_GrabComponent.AttachComponents` (`self.BP_GrabComponent`) (delegate `UpdateGrab`))
  (bind _asbp_main_player (cast `/Game/Blueprints/BP_MainPlayer` (`GameplayStatics.GetPlayerPawn` 0)))
  (set `self.PlayerREF` _asbp_main_player))

(event `UpdateGrab`
  (bind _regularmesh (`self.RegularMesh`))
  (if (`/Game/Blueprints/BP_GrabComponent.Is Grabbing` (`self.BP_GrabComponent`))
    (`SceneComponent.K2_DetachFromComponent` _regularmesh "KeepWorld" "KeepWorld" "KeepWorld" true)
    (bind _output_get (set `self.NewVar` (`SceneComponent.K2_GetComponentLocation` _regularmesh)))
    (`ActorComponent.K2_DestroyComponent` _regularmesh)
    (bind _returnvalue (`AddComponent|NODE_AddGeometryCollectionComponent-0` :`RelativeTransform` (`KismetMathLibrary.MakeTransform` _output_get (struct) (8.0 8.0 8.0))))
    (`GeometryCollectionComponent.SetRestCollection` _returnvalue "/Game/_Art/GeometryCollections/FlowerPot.FlowerPot")
    (`KismetSystemLibrary.PrintString` "Hello")
    (else
      (`SceneComponent.K2_AttachToComponent` _regularmesh (`/Game/Blueprints/BP_MainPlayer.Camera` (`self.PlayerREF`)) "None" "KeepWorld" "KeepWorld" "KeepWorld" false))))

(fn `UserConstructionScript`)