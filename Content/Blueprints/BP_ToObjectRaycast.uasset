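; BP_ToObjectRaycast tests whether a component is visible to the first player, given vertex offsets from its world location.
; A screen-projection pre-check requires at least one vertex inside the viewport.
; Line traces against WorldStatic then run from the camera to each vertex, nudged slightly toward the component's origin to ensure contact.
; Any first hit on the component itself, or on one tagged "Marker", counts as visible.
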(fn `Is Component Visible`
  (params (Vertices :type "Array of Vector Structure") (Component :type "StaticMeshComponent Object Reference"))
  (returns (IsVisible :type Boolean))
  (bind _returnvalue (`SceneComponent.K2_GetComponentLocation` Component))
  (bind _infov (`self.IsComponentInFOV` Vertices Component))
  (if _infov
    (for _array_element Vertices
      (bind _returnvalue_2 (+ _array_element _returnvalue))
      (bind (_outhit _returnvalue_3) (`KismetSystemLibrary.LineTraceSingleForObjects` :`Start` (`Actor.K2_GetActorLocation` (`GameplayStatics.GetPlayerCameraManager` null)) :`End` (+ _returnvalue_2 (* (`KismetMathLibrary.Normal` (- _returnvalue _returnvalue_2)) 2)) :`ObjectTypes` (`|MakeArray` "ObjectTypeQuery1" :!type "EObjectTypeQuery Enum") :`bIgnoreSelf` false :`DrawTime` 0.5))
      (if _returnvalue_3
        (bind (_bblockinghit _binitialoverlap _time _distance _location _impactpoint _normal _impactnormal _physmat _hitactor _hitcomponent) (`GameplayStatics.BreakHitResult` _outhit))
        (if (== _hitcomponent (`local.Component`))
          (return true)
          (elif (`ActorComponent.ComponentHasTag` _hitcomponent "Marker")
            (return true)))))
    (return false)
    (else
      (return false))))

(fn `IsComponentInFOV`
  (params (Vertices :type "Array of Vector Structure") (Component :type "StaticMeshComponent Object Reference"))
  (returns (InFOV :type Boolean))
  (for _array_element Vertices
    (bind _infov (`self.IsPointInFOV` (+ _array_element (`SceneComponent.K2_GetComponentLocation` Component))))
    (if _infov
      (return true)))
  (return false))

(fn `IsPointInFOV`
  (params (Point :type "Vector Structure"))
  (returns (InFOV :type Boolean))
  (bind (_returnvalue_x _returnvalue_y) (`KismetMathLibrary.BreakVector2D` (`WidgetLayoutLibrary.GetViewportSize` null)))
  (bind _screenlocation (`PlayerController.ProjectWorldLocationToScreen` (`GameplayStatics.GetPlayerController` null) Point false))
  (return (and (> (`KismetMathLibrary.BreakVector2D` _screenlocation) 0.0) (> (`.Y` (`KismetMathLibrary.BreakVector2D` _screenlocation)) 0.0) (< (`KismetMathLibrary.BreakVector2D` _screenlocation) _returnvalue_x) (< (`.Y` (`KismetMathLibrary.BreakVector2D` _screenlocation)) _returnvalue_y))))