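; BP_PlayerTrigger is a box trigger that signals other objects when a Character enters or, optionally, leaves it.
; On begin overlap it calls UpdateMessage on every element of its Output array with one enum value.
; When UseEndOverlap is set, end overlap sends a second value to the same elements.
; The construction script sizes the box from the Scale variable.
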(event `self.ReceiveActorBeginOverlap`
  (params (OtherActor :type "Actor Object Reference"))
  (cast `Character` OtherActor)
  (for _array_element (`self.Output`)
    (message `/Game/Blueprints/BI_Signal.Update` _array_element "NewEnumerator0")))

(event `self.ReceiveActorEndOverlap`
  (params (OtherActor :type "Actor Object Reference"))
  (if (`self.UseEndOverlap?`)
    (cast `Character` OtherActor)
    (for _array_element (`self.Output`)
      (message `/Game/Blueprints/BI_Signal.Update` _array_element "NewEnumerator1"))))

(fn `UserConstructionScript`
  (`BoxComponent.SetBoxExtent` (`self.Box`) (`self.Scale`) true))