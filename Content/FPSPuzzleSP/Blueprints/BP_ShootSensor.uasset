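; BP_ShootSensor is a puzzle sensor that reacts to being hit by a projectile.
; On a hit it sends an update message to every target in its OutputTo list, playing a data-table sound attached to its Cube inside that loop.
; When TimerEnable is set, a one-shot timer later sends the opposite message to the same targets after TimerDelay.
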(event `/Game/FPSPuzzleSP/Blueprints/Components/BI_ProjectileHit.ProjectileHit`
  (for _array_element (`self.Output to:`)
    (message `/Game/Blueprints/BI_Signal.Update` _array_element "NewEnumerator0")
    (`/Game/FPSPuzzleSP/Blueprints/Components/FL_PuzzleLib.PlaySoundByDataTable_Attached` "BP_ShootSensor" 0.8 (`self.Cube`))
    (if (`self.Timer enable`)
      (`KismetSystemLibrary.K2_SetTimerDelegate` (delegate `ret_off`) (`self.Timer Delay`)))))

(event `ret_off`
  (for _array_element (`self.Output to:`)
    (message `/Game/Blueprints/BI_Signal.Update` _array_element "NewEnumerator1")))

(fn `UserConstructionScript`)