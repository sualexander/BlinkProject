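; BP_ImpulsePanel is a launch panel that flings characters and physics objects that overlap its trigger.
; An On/Off signal toggles whether the panel is active, reusing the AvailibleFromStart flag.
; Characters get LaunchCharacter, while BP_PhysicObjectBase actors and their children have their mesh's physics linear velocity changed, with VelocityChange choosing between overriding and adding the Impulse.
; Either launch plays a data-table sound at the panel.
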(event `/Game/Blueprints/BI_Signal.Update`
  (params (Signal :type "/Game/FPSPuzzleSP/Blueprints/Components/Enum_Signal Enum" :default "NewEnumerator0"))
  (switch `/Game/FPSPuzzleSP/Blueprints/Components/Enum_Signal` Signal
    (:`NewEnumerator0`
      (set `self.Availible From Start` true))
    (:`NewEnumerator1`
      (set `self.Availible From Start` false))))

(event `self.Trigger.OnComponentBeginOverlap`
  (params (OverlappedComponent :type "PrimitiveComponent Object Reference") (OtherActor :type "Actor Object Reference") (OtherComp :type "PrimitiveComponent Object Reference") (OtherBodyIndex :type Integer) (bFromSweep :type Boolean) (SweepResult :type "HitResult Structure (by ref)"))
  (bind _velocity_change (`self.Velocity Change`))
  (if (`self.Availible From Start`)
    (`|ExecutionSequence`
      (:`then_0`
        (bind _ascharacter (cast `Character` OtherActor))
        (`Character.LaunchCharacter` _ascharacter (`self.Impulse`) _velocity_change _velocity_change))
      (:`then_1`
        (bind _asbp_physic_object_base (cast `/Game/FPSPuzzleSP/Blueprints/BP_PhysicObjectBase` OtherActor)) ; It will works with all childrens of this class.
        (`PrimitiveComponent.SetAllPhysicsLinearVelocity` (`/Game/FPSPuzzleSP/Blueprints/BP_PhysicObjectBase.Mesh` _asbp_physic_object_base) (`self.Impulse`) (not (`self.Velocity Change`)))))
    (`/Game/FPSPuzzleSP/Blueprints/Components/FL_PuzzleLib.PlaySoundByDataTable` "BP_ImpulsePanel" (`self.K2_GetActorLocation`) 0.7)))

(fn `UserConstructionScript`)